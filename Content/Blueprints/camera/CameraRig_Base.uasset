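; CameraRig_Base is a camera rig actor that follows an Alt tracker's transform every tick and positions its Pupil component relative to it.
; Pupil uses the optic-line transform with X offset and correction, or in test mode a spawned second Alt's pose relative to the rig.
; A helper widget displays tracking poses and restarts tracking on click.
; A fixed-length frame-delay buffer is maintained, but the applied transform is undelayed.
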(event Custom|restartTrack
  (bind _bp_alttrackertag (Variables|Default|GetBP_AltTrackerTag))
  (Default|StartTrackingTask _bp_alttrackertag (Variables|/AntilatencyTracking/Blueprints/Samples/SceneComponents/BP_AltTracker.BP_AltTracker_C|GetcurentNode _bp_alttrackertag)))

(event EventBeginPlay
  (Utilities|FlowControl|Sequence
    (:then_0
      (for _index (range 0 (Variables|Default|GetFramesDelayNum))
        (Utilities|Array|Add (Variables|Default|GetDelayArr) (Math|Transform|MakeTransform "0, 0, 0"))))
    (:then_1
      (bind _returnvalue (UserInterface|CreateWidget "/Game/Blueprints/altWidget.altWidget_C" (Game|GetPlayerController 0)))
      (UserInterface|Viewport|AddtoViewport _returnvalue 0)
      (bind _output_get (Variables|Default|SetHelperWidget _returnvalue))
      (EventDispatchers|BindEventtoClickRestart _output_get (delegate Custom|restartTrack))
      (if (Variables|Default|GetuseTestAlt)
        (bind _returnvalue_2 (Game|SpawnActorfromClass "/Game/Blueprints/camera/alt2.alt2_C" (Math|Transform|MakeTransform "0, 0, 0" "0, 0, 0" "1,1,1") "Undefined" 0 0))
        (Variables|Default|Setalt2 _returnvalue_2)))))

(event Collision|EventActorBeginOverlap
  (params (OtherActor :type Actor%20Object%20Reference)))

(event EventTick
  (params (DeltaSeconds :type Float%20%28single-precision%29))
  (bind _returnvalue (Transformation|GetActorTransform))
  (bind _bp_alttrackertag (Variables|Default|GetBP_AltTrackerTag))
  (bind _transformopticline (Variables|Default|GettransformOpticLine))
  (bind _alt2 (Variables|Default|Getalt2))
  (bind _alt2_2 (Variables|Default|Getalt2))
  (bind _correcttransform (Variables|Default|GetcorrectTransform))
  (bind _pupil (Variables|Default|GetPupil))
  (bind _pupiloffsetx (Variables|Default|GetpupilOffsetX))
  (bind (_location _rotation) (Math|Transform|BreakTransform _transformopticline))
  (bind (_location_2 _rotation_2) (Math|Transform|BreakTransform _correcttransform))
  (bind _returnvalue_2 (Transformation|GetActorTransform _alt2_2))
  (bind _returnvalue_3 (Math|Transform|InvertTransform _returnvalue))
  (bind _trackingtransform (Variables|/AntilatencyTracking/Blueprints/Samples/SceneComponents/BP_AltTracker.BP_AltTracker_C|GetTrackingTransform _bp_alttrackertag))
  (bind _bp_alttrackertag_2 (Variables|/Game/Blueprints/camera/alt2.alt2_C|GetBP_AltTrackerTag _alt2))
  (bind _returnvalue_4 (Utilities|String|ToString(Vector) (.location _trackingtransform)))
  (bind _returnvalue_5 (Utilities|String|ToString(Rotator) (.rotation _trackingtransform)))
  (bind (_x _y _z) (Math|Vector|BreakVector _location))
  (bind _returnvalue_6 (Math|Transform|ComposeTransforms _returnvalue_2 _returnvalue_3))
  (bind _trackingtransform_2 (Variables|/AntilatencyTracking/Blueprints/Samples/SceneComponents/BP_AltTracker.BP_AltTracker_C|GetTrackingTransform _bp_alttrackertag_2))
  (bind _returnvalue_7 (- _x _pupiloffsetx))
  (bind _returnvalue_8 (Math|Vector|MakeVector _returnvalue_7 _y _z))
  (bind _returnvalue_9 (Math|Transform|MakeTransform _returnvalue_8 _rotation))
  (bind (_location_3 _rotation_3) (Math|Transform|BreakTransform _returnvalue_9))
  (Utilities|FlowControl|Sequence
    (:then_0
      (Utilities|Array|Add (Variables|Default|GetDelayArr) (Variables|/AntilatencyTracking/Blueprints/Samples/SceneComponents/BP_AltTracker.BP_AltTracker_C|GetTrackingTransform (Variables|Default|GetBP_AltTrackerTag))))
    (:then_1
      (Transformation|SetActorTransform (Math|Transform|MakeTransform (.location _trackingtransform) (.rotation _trackingtransform) "1,1,1"))
      (Default|UpdateInfo (Variables|Default|GetHelperWidget) _returnvalue_4 _returnvalue_5)
      (if (Variables|Default|GetuseTestAlt)
        (Transformation|SetRelativeTransform _pupil _returnvalue_6 false false)
        (Variables|Default|SetcurrentTransformOpticLine _returnvalue_6)
        (Default|UpdateInfo (Variables|Default|GetHelperWidget) _returnvalue_4 _returnvalue_5 (Utilities|String|ToString(Vector) (.location _trackingtransform_2)) (Utilities|String|ToString(Rotator) (.rotation _trackingtransform_2)))
        (else
          (Transformation|SetRelativeTransform _pupil (Math|Transform|MakeTransform (+ _location_3 _location_2) (Math|Rotator|CombineRotators _rotation_3 _rotation_2)) false false)
          (Variables|Default|SetpupilDebugWorldTransfrom (Transformation|GetWorldTransform (Variables|Default|GetPupil))))))
    (:then_2
      (Utilities|Array|RemoveIndex (Variables|Default|GetDelayArr)))))

(fn ConstructionScript)
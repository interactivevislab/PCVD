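; CameraRig is a camera actor that follows the transform produced by BPAltTracker.
; Every tick it copies the tracker's location, pitch and yaw, forcing roll to zero to keep the view level.
; On BeginPlay it adds an AltWidget to the viewport and binds its restart click to restart tracking from the tracker's current node.
; Widget updates for tracking info and camera transform exist but are disconnected.
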(event Custom|restartTrack
  (bind _bp_alttracker (Variables|Default|GetBP_AltTracker))
  (Default|StartTrackingTask _bp_alttracker (Variables|/AntilatencyTracking/Blueprints/Samples/SceneComponents/BP_AltTracker.BP_AltTracker_C|GetcurentNode _bp_alttracker)))

(event EventBeginPlay
  (bind _returnvalue (UserInterface|CreateWidget "/Game/Blueprints/altWidget.altWidget_C" (Game|GetPlayerController 0)))
  (UserInterface|Viewport|AddtoViewport _returnvalue 0)
  (bind _output_get (Variables|Default|SetHelperWidget _returnvalue))
  (EventDispatchers|BindEventtoClickRestart _output_get (delegate Custom|restartTrack)))

(event Collision|EventActorBeginOverlap
  (params (OtherActor :type Actor%20Object%20Reference)))

(event EventTick
  (params (DeltaSeconds :type Float%20%28single-precision%29))
  (bind _bp_alttracker (Variables|Default|GetBP_AltTracker))
  (bind _trackingtransform (Variables|/AntilatencyTracking/Blueprints/Samples/SceneComponents/BP_AltTracker.BP_AltTracker_C|GetTrackingTransform _bp_alttracker))
  (bind (_location _rotation) (Math|Transform|BreakTransform _trackingtransform))
  (bind (_roll _pitch _yaw) (Math|Rotator|BreakRotator _rotation))
  (Transformation|SetActorTransform (Math|Transform|MakeTransform _location (Math|Rotator|MakeRotator 0.0 _pitch _yaw) "1,1,1")))

(fn ConstructionScript)
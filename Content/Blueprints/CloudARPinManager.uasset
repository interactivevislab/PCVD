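; Multiplayer Cloud AR pin manager that anchors a shared ARSceneRoot through a validated game-state machine with widget status messages.
; The authority finds a plane, pins the root on touch, then manually hosts it to set the CloudID.
; Clients await that ID and switch to Resolving, but resolving only runs through manual load by ID.
; Saving attaches the grid via the player controller using the adjusted room transform and displays the ID; the save-to-slot code is unwired.
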(event Custom|ManualHostARPin
  (Utilities|ManualHostCloudARPin
    (:Success
      (Default|ToggleHostButton (Variables|Default|GetCloudARPinWidget) false)
      (bind _asbp_player_controller_atbtt (Utilities|Casting|CastToBP_PlayerController_ATBTT (Game|GetPlayerController 0))))
    (:Failed
      (Development|PrintString "Manual host failed!" true true "(R=1.000000,G=0.000000,B=0.020423,A=1.000000)"))))

(event Custom|SaveARState
  (bind _arsceneroot (Variables|Default|GetARSceneRoot))
  (bind _cloudid (Variables|/Game/Blueprints/MultiplayerARSceneRoot.MultiplayerARSceneRoot_C|GetCloudID _arsceneroot))
  ;[1 1 1] Save ARPin information on server
  (bind _asbp_player_controller_atbtt (Utilities|Casting|CastToBP_PlayerController_ATBTT (Game|GetPlayerController 0)))
  (Default|ServerAttachGrid _asbp_player_controller_atbtt 0 (Variables|Default|GetAdjustedRoomTransform))
  (Development|PrintString (Utilities|String|Append "SaveArPin  id  ==  " _cloudid) true true "(R=1.000000,G=0.000000,B=0.000000,A=1.000000)" 1e+01)
  (Default|SetSaveId (Variables|Default|GetCloudARPinWidget) (Utilities|Text|ToText(String) _cloudid)))

(event Custom|LoadARState
  (params (ArPinId :type String))
  (Variables|Default|SetCurrentGameState "NewEnumerator3")
  (Utilities|ManualLoadCloudARPin ArPinId
    (:Failed
      (Development|PrintString "Fail after load"))
    (:SuperFail
      (Development|PrintString "Super Fail after load"))))

(event EventBeginPlay
  (bind _simulatedplane (Variables|Default|GetSimulatedPlane))
  (Utilities|IsARSupportedPlatform
    (:true
      (Rendering|SetActorHiddenInGame _simulatedplane true)
      (Development|PrintString "StartARMODULE!!!!!!")
      ;[1 1 1] Wait the ARPlayerController to create the UIWidget and get the reference
      (Utilities|FlowControl|Delay 0.2)
      (bind _asbp_player_controller_atbtt (Utilities|Casting|CastToBP_PlayerController_ATBTT (Game|GetPlayerController 0)))
      (bind _output_get (Variables|Default|SetCloudARPinWidget (Variables|/Game/AdvancedTurnBasedTileToolkit/Core/BP_PlayerController_ATBTT.BP_PlayerController_ATBTT_C|GetCloudARPinWidget _asbp_player_controller_atbtt)))
      (EventDispatchers|BindEventtoOnHostAttempt _output_get (EventDispatchers|CreateEvent :!event Custom|ManualHostARPin))
      (EventDispatchers|BindEventtoOnSaveAttempt _output_get (EventDispatchers|CreateEvent :!event Custom|SaveARState))
      (EventDispatchers|BindEventtoOnLoadAttempt _output_get (EventDispatchers|CreateEvent :!event Custom|LoadARState))
      (Development|PrintString "BindForArEvent")
      (Networking|SwitchHasAuthority
        (:Authority
          _)
        (:Remote
          ;[1 1 1] Find and set the ARSceneRoot actor spawned by the server
          (bind _outactors (Actor|GetAllActorsOfClass "/Game/Blueprints/MultiplayerARSceneRoot.MultiplayerARSceneRoot_C"))
          (Variables|Default|SetARSceneRoot (Utilities|Array|Get(acopy) _outactors))))
      ;[1 1 1] Set the initial game state for server and client
      (bind _asgi_avatar_game_instance (Utilities|Casting|CastToGI_AvatarGameInstance (Game|GetGameInstance)))
      (Variables|Default|SetARGameInstance _asgi_avatar_game_instance)
      (if (Ability|HasAuthority)
        (Utilities|TransitiontoGameState "NewEnumerator4")
        (else
          (Utilities|TransitiontoGameState "NewEnumerator1"))))
    (:false
      (Rendering|SetActorHiddenInGame _simulatedplane false))))

(event EventTick
  (params (DeltaSeconds :type Float%20%28single-precision%29))
  ;[1 1 1] Tick the Actor based on the current game state
  (switch Utilities|FlowControl|Switch|SwitchonCloudARPinGameState (Variables|Default|GetCurrentGameState)
    (:NewEnumerator4
      (Utilities|CheckARPlaneDetected))
    (:NewEnumerator1
      (Utilities|CheckCloudIDSynced))))

(event Input|TouchEvents|InputTouch
  (params (Location :type Vector) (FingerIndex :type ETouchIndex%20Enum))
  (:Pressed
    (Development|PrintString "Touch from Cloud manager")
    ;[1 1 1] Handle touch event based on the current game state
    (switch Utilities|FlowControl|Switch|SwitchonCloudARPinGameState (Variables|Default|GetCurrentGameState)
      (:NewEnumerator0
        (Utilities|HostCloudARPinRoot FingerIndex)))))

(fn ConstructionScript)

(fn GetCloudARPinError
  (params (CloudPin :type Cloud%20AR%20Pin%20Object%20Reference) (TaskResult :type EARPinCloudTaskResult%20Enum :default "Success"))
  (if (Utilities|IsValid CloudPin)
    (return (Utilities|String|EnumtoString (Class|CloudARPin|GetARPinCloudState CloudPin)))
    (else
      (return (Utilities|String|EnumtoString TaskResult)))))

(fn GetRelativeTransfromtoARSceneRoot
  (params (ChildActorWorldTransform :type Transform))
  (bind _arsceneroot (Variables|Default|GetARSceneRoot))
  (bind _cloudarpinroot (Variables|/Game/Blueprints/MultiplayerARSceneRoot.MultiplayerARSceneRoot_C|GetCloudARPinRoot _arsceneroot))
  (bind _returnvalue (Transformation|GetWorldTransform _cloudarpinroot))
  (return (Math|Transform|MakeTransform (Math|Transform|InverseTransformLocation _returnvalue (.location ChildActorWorldTransform)) (Math|Transform|InverseTransformRotation _returnvalue (.rotation ChildActorWorldTransform)))))

(fn MoveRoom
  (params (Location :type Vector))
  (bind _roomactor (Variables|Default|GetRoomActor))
  (bind _scene (Variables|/Game/Blueprints/BP_ActorRoom.BP_ActorRoom_C|GetScene _roomactor))
  (Utilities|IsValid _roomactor
    (:Is%20Valid
      (Transformation|SetRelativeLocation _scene (+ (Variables|/Script/Engine.SceneComponent|GetRelativeLocation _scene) Location) false false)
      (Variables|Default|SetAdjustedRoomTransform (Transformation|GetRelativeTransform (Variables|/Game/Blueprints/BP_ActorRoom.BP_ActorRoom_C|GetScene (Variables|Default|GetRoomActor)))))))

(fn RotateRoom
  (params (Rotation :type Rotator))
  (bind _roomactor (Variables|Default|GetRoomActor))
  (bind _scene (Variables|/Game/Blueprints/BP_ActorRoom.BP_ActorRoom_C|GetScene _roomactor))
  (bind _relativerotation (Variables|/Script/Engine.SceneComponent|GetRelativeRotation _scene))
  (Utilities|IsValid _roomactor
    (:Is%20Valid
      (Transformation|SetRelativeRotation _scene (Math|Rotator|MakeRotator (+ (.roll Rotation) (.roll _relativerotation)) (+ (.pitch Rotation) (.pitch _relativerotation)) (+ (.yaw Rotation) (.yaw _relativerotation))) false false)
      (Variables|Default|SetAdjustedRoomTransform (Transformation|GetRelativeTransform (Variables|/Game/Blueprints/BP_ActorRoom.BP_ActorRoom_C|GetScene (Variables|Default|GetRoomActor)))))))

(fn ScaleRoom)

(fn FrezeArSceneRoot
  (Variables|/Game/Blueprints/MultiplayerARSceneRoot.MultiplayerARSceneRoot_C|SetCanMove (Variables|Default|GetARSceneRoot) false))

(fn RemoveArPin
  (Utilities|RemovePinifValid))
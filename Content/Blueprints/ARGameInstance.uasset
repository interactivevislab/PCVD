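; Game instance for an AR game that hosts and joins two-player LAN sessions, opening ARGameMap as a listen server.
; Clients join through a session search result or a console open command to a typed IP.
; IP joins count as failed if MainMenu is still loaded after a delay.
; Errors share one reused dialog widget; the IP check only range-checks four-part dotted input and accepts anything else.
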(event Custom|JoinSelectedServer
  (params (SearchResult :type Blueprint%20Session%20Result%20Structure%20%28by%20ref%29))
  (|JoinSession (Game|GetPlayerController 0) SearchResult))

(event Custom|Join%20Session%20Via%20IP
  (params (ServerIPAddress :type String))
  ;[1 1 1] Join the session using the input IP address
  (bind _isvalid (CallFunction|IsValidIPAddress ServerIPAddress))
  (if _isvalid
    (Development|ExecuteConsoleCommand (Utilities|String|Append "open " ServerIPAddress) 0)
    (Utilities|FlowControl|Delay 5.0)
    (bind _returnvalue (Game|GetCurrentLevelName true))
    (if (Utilities|Enum|Equal(Enum) _returnvalue "MainMenu")
      (CallFunction|ShowDialog (Utilities|Text|ToText(String) (Utilities|String|Append "Failed to join the session hosted at IP: " ServerIPAddress))))
    (else
      (CallFunction|ShowDialog "Invalid IP Address"))))

(event Custom|StartSession
  ;[1 1 1] Create network session and open the game level in listen mode
  (|Session (Game|GetPlayerController 0) 2 true
    (:then
      (Variables|Default|SetRoomID (Class|CloudARPinUtils|GetHostSessionId))
      (Game|OpenLevel(byName) "ARGameMap" true "?Listen"))
    (:OnFailure
      (CallFunction|ShowDialog "Failed to create session."))))

(event Custom|JoinSession
  (params (Session :type Blueprint%20Session%20Result%20Structure))
  ;[1 1 1] Search for hosted session and join the first one if the IP input box is blank.
  (|JoinSession (Game|GetPlayerController 0) Session
    (:OnFailure
      (CallFunction|ShowDialog "Failed to join the session."))))

(fn ShowDialog
  (params (Message :type Text))
  (Utilities|IsValid (Variables|Default|GetErrorDialog)
    (:Is%20Valid
      (Widget|SetVisibility (Variables|Default|GetErrorDialog) "Visible"))
    (:Is%20Not%20Valid
      (bind _returnvalue (UserInterface|CreateWidget "/Game/Blueprints/MessageDialog.MessageDialog_C"))
      (bind _output_get (Variables|Default|SetErrorDialog _returnvalue))
      (UserInterface|Viewport|AddtoViewport _output_get 0)))
  (Variables|/Game/Blueprints/MessageDialog.MessageDialog_C|SetMessage _output_get Message))

(fn IsValidIPAddress
  (params (SourceString :type String))
  (bind _returnvalue (Utilities|String|ParseIntoArray SourceString "."))
  (if (== (Utilities|Array|Length _returnvalue) 4)
    (for _array_element _returnvalue
      (if (not (Math|Integer|InRange(Integer) (Math|Conversions|ToInteger(Byte) _array_element) 0 255))
        (return false)))
    (return true)
    (else
      (return (>= (Utilities|Array|Length (Utilities|String|ParseIntoArray SourceString ":")) 0)))))

(fn GetPower
  (return 0))
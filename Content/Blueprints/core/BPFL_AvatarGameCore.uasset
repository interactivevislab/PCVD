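; Blueprint function library for the avatar game core that gives access to the GameManager and to player info by faction.
; GetGameManager finds the GameManager actor in the world with GetActorOfClass.
; GetPlayerInfoFromFraction finds the faction's index in FactionPlayerInGame and returns the PlayersInGame entry at that same index, relying on parallel arrays.
; An unknown faction only prints an error string.
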(fn GetGameManager
  (bind _returnvalue (Actor|GetActorOfClass (LocalVariables|Get__WorldContext) "/Game/Blueprints/GameManager.GameManager_C"))
  (return _returnvalue))

(fn GetPlayerInfofromFraction
  (params (NewParam :type EFaction%20Enum :default "NewEnumerator3"))
  (bind ___worldcontext (LocalVariables|Get__WorldContext))
  (bind _gamemanager (CallFunction|GetGameManager ___worldcontext))
  (bind _factionplayeringame (Variables|/Game/Blueprints/GameManager.GameManager_C|GetFactionPlayerInGame _gamemanager))
  (if (Utilities|Array|ContainsItem _factionplayeringame NewParam)
    (return (Utilities|Array|Get(acopy) (Variables|/Game/Blueprints/GameManager.GameManager_C|GetPlayersInGame _gamemanager) (Utilities|Array|FindItem _factionplayeringame NewParam)))
    (else
      (Development|PrintString (LocalVariables|Get__WorldContext) "ERROR FRACTION DONT FIND"))))
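; Game mode that handles player sign-in through the Avatar API manager, then opens LobbyLevel.
; Windows shows the authorization widget with a spectator button; other platforms try a refresh token first, falling back to the widget.
; Successful auth sets the player type on the game instance, fetches user info and picks mesh and icon from hardcoded ISU IDs.
; A skip-auth path injects a dev user and goes straight to the lobby.
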(event Custom|AuthFromRefreshTokenCpmplete
  (params (Success :type Boolean) (refreshToken :type String) (accessToken :type String) (error :type String))
  (if Success
    (CallFunction|AuthSuccess)
    (else
      (CallFunction|ShowAuthWidget))))

(event Custom|ShowAuthWidget
  (bind _returnvalue (Game|GetPlayerController 0))
  (bind _returnvalue_2 (UserInterface|CreateWidget "/Game/Blueprints/UI/WBP_AuthorizationScreen.WBP_AuthorizationScreen_C" _returnvalue))
  (UserInterface|Viewport|AddtoViewport _returnvalue_2 0)
  (Input|SetInputModeUIOnly _returnvalue _returnvalue_2 "LockAlways")
  (Variables|Default|SetauthWidget _returnvalue_2)
  (Variables|/Script/Engine.PlayerController|SetbShowMouseCursor _returnvalue true)
  (EventDispatchers|BindEventtoClickOk (Variables|Default|GetauthWidget) (EventDispatchers|CreateEvent :!event Custom|TryAuthFromUserCredentials))
  (Input|SetInputModeUIOnly (Game|GetPlayerController 0) (Variables|Default|GetauthWidget) "DoNotLock")
  (EventDispatchers|BindEventtoClickSkipAuth (Variables|Default|GetauthWidget) (EventDispatchers|CreateEvent :!event Custom|skipAuth)))

(event Custom|TryAuthFromUserCredentials
  (params (Login :type String) (Pass :type String))
  (Class|AvatarApiManager|AuthfromUserCredential (Variables|Default|GetAvatarAPIManager) Login Pass (delegate Custom|AuthFromUserCredentialComplete)))

(event Custom|AuthFromUserCredentialComplete
  (params (Success :type Boolean) (refreshToken :type String) (accessToken :type String) (error :type String))
  (if Success
    (CallFunction|AuthSuccess)
    (else
      (CallFunction|ShowWidgetError error))))

(event Custom|ShowWidgetError
  (params (NewParam :type String))
  (Default|ShowErrorMessage (Variables|Default|GetauthWidget) NewParam))

(event Custom|AuthSuccess
  (bind _asgi_avatar_game_instance (Utilities|Casting|CastToGI_AvatarGameInstance (Game|GetGameInstance)))
  (Default|SetPlayerType _asgi_avatar_game_instance "NewEnumerator0")
  (Development|PrintString "AuthSucces")
  (Class|AvatarApiManager|GetUserInfofromAvatarAPI (Variables|Default|GetAvatarAPIManager) (delegate Custom|getUserInfoComplete)))

(event Custom|getUserInfoComplete
  (params (userInfo :type User%20Info%20Structure))
  (CallFunction|GetUserMesh)
  (Game|OpenLevel(byName) "LobbyLevel"))

(event Custom|getUserMesh
  (bind _avatarapimanager (Variables|Default|GetAvatarAPIManager))
  (bind _returnvalue (Class|AvatarApiManager|GetUserInfo (Variables|Default|GetAvatarAPIManager)))
  (switch string (Utilities|String|ToString(Integer) (.isu_id _returnvalue))
    (:Default
      (Class|AvatarApiManager|ChangeStaticMeshforUser _avatarapimanager "/Game/Meshes/Misha/SK_Misha_default.SK_Misha_default")
      (Class|AvatarApiManager|ChangeUserIcon _avatarapimanager "/Game/AdvancedTurnBasedTileToolkit/Units/T_UnitIcon_Default.T_UnitIcon_Default"))
    (:287357
      (Class|AvatarApiManager|ChangeStaticMeshforUser _avatarapimanager "/Game/Meshes/Dima/SK_Dima.SK_Dima")
      (Class|AvatarApiManager|ChangeUserIcon _avatarapimanager "/Game/Icons/avatar_test/avatarDima.avatarDima"))
    (:311335
      (Class|AvatarApiManager|ChangeStaticMeshforUser _avatarapimanager "/Game/Meshes/Misha/SK_Misha.SK_Misha")
      (Class|AvatarApiManager|ChangeUserIcon _avatarapimanager "/Game/Icons/avatar_test/avatarMisha.avatarMisha"))))

(event Custom|skipAuth
  (Class|AvatarApiManager|SetUserInfoDev (Variables|Default|GetAvatarAPIManager) (Utilities|Struct|MakeUserInfo "Viz" "Lab" 0 1111 "/Game/Meshes/Dima/SK_Dima.SK_Dima" 0))
  (Game|OpenLevel(byName) "LobbyLevel"))

(event EventBeginPlay
  (Utilities|IsWin
    (:true
      (Variables|Default|SetAvatarAPIManager (CallFunction|GetApiManager))
      ;[1 1 1] PC AUTH
      (CallFunction|ShowAuthWidget)
      (Widget|SetVisibility (Variables|/Game/Blueprints/UI/WBP_AuthorizationScreen.WBP_AuthorizationScreen_C|GetButton_SpectatorMode (Variables|Default|GetauthWidget)) "Visible"))
    (:false
      (bind _output_get (Variables|Default|SetAvatarAPIManager (CallFunction|GetApiManager)))
      (Class|AvatarApiManager|TryAuthfromRefreshToken _output_get (delegate Custom|AuthFromRefreshTokenCpmplete)))))

(fn ConstructionScript)
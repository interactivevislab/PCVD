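; Blueprint function library that gives static access to the avatar API manager and the user's avatar data.
; GetApiManager casts the game instance to GI_AvatarGameInstance and returns its AvatarAPIManager.
; GetUserInfo queries that manager, and GetUserMesh returns the UserMesh field of the result.
; GetUserPower is an empty stub.
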(fn GetApiManager
  (bind _asgi_avatar_game_instance (Utilities|Casting|CastToGI_AvatarGameInstance (Game|GetGameInstance (LocalVariables|Get__WorldContext))))
  (return (Variables|/Game/Blueprints/core/GI_AvatarGameInstance.GI_AvatarGameInstance_C|GetAvatarAPIManager _asgi_avatar_game_instance)))

(fn GetUserInfo
  (bind _returnvalue (Class|AvatarApiManager|GetUserInfo (CallFunction|GetApiManager (LocalVariables|Get__WorldContext))))
  (return _returnvalue))

(fn GetUserPower)

(fn GetUserMesh
  (bind _userinfo (CallFunction|GetUserInfo (LocalVariables|Get__WorldContext)))
  (return (.userMesh (Utilities|Struct|BreakUserInfo _userinfo))))
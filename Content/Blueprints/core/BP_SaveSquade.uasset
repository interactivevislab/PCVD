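; BP_SaveSquade holds saved squad data in three numbered slots.
; A setter and a getter switch on the slot number to write or read the matching slot variable.
; An existence check reuses the getter and reports a slot as filled when its contents have non-zero length.
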(fn SetSaveSquadSLot
  (params (Input :type Array%20of%20ST%20Soldier%20Structures) (slot :type Integer))
  (switch int slot
    (:1
      (Variables|Default|SetSlot_1 Input))
    (:2
      (Variables|Default|SetSlot_2 Input))
    (:3
      (Variables|Default|SetSlot_3 Input))))

(fn GetSquadSlot
  (params (slot :type Integer))
  (switch int slot
    (:1
      (return (Variables|Default|GetSlot_1)))
    (:2
      (return (Variables|Default|GetSlot_2)))
    (:3
      (return (Variables|Default|GetSlot_3)))))

(fn CheckSlotExist
  (params (slot :type Integer))
  (return (!= (Utilities|Array|Length (CallFunction|GetSquadSlot slot)) 0)))
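; BP_unit_avatar is a unit Blueprint that handles what happens when the unit is selected in the turn-based game.
; Selection asks the turn manager whether activation is allowed and reports the unit as selected, making it active only if permitted.
; An allowed unit leaves the grid manager's big-unit array, activates its default ability and, with an ability system component, refreshes the ability box and queued actions.
; Otherwise the active player shows the enemy display ability.
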(event Custom|activateDefaultAbility
  (bind _self self)
  (bind _returnvalue (Components|GetOwner _self))
  (Class|BPIAbility|ActivateAbility(Message) (select (Utilities|IsValid _returnvalue) _returnvalue (Game|GetPlayerController 0)) (Variables|Default|GetDefaultAbility) self))

(event EventBeginPlay
  (|CallParentFunction) ; This node is disabled and will not be called.\nDrag off pins to build functionality.
)

(event Collision|EventActorBeginOverlap
  (params (OtherActor :type Actor%20Object%20Reference)))

(event EventSelectActor
  (bind _turnmanager (Utilities|GetTurnManager))
  (bind _ballowed (Default|CheckifUnitActivationAllowed _turnmanager self))
  (Default|RunonActorSelected _turnmanager self _ballowed)
  (if _ballowed
    (Default|RemoveUnitfromBigUnitArray (Variables|Default|GetGridManagerRef) self)
    (CallFunction|ActivateDefaultAbility)
    (if (Utilities|IsValid (Actor|GetComponentbyClass self "/Game/AdvancedTurnBasedTileToolkit/Core/Units/BP_AbilitySystem.BP_AbilitySystem_C"))
      (bind _turnmanager_2 (Utilities|GetTurnManager))
      (Default|UpdateAbilityBox _turnmanager_2 self)
      (bind _actionmanager (Utilities|GetActionManager))
      (Default|InitializeQueuedActions _actionmanager))
    (else
      (Class|BPIAbility|ActivateAbility(Message) (Variables|/Game/AdvancedTurnBasedTileToolkit/Core/BP_TurnManager.BP_TurnManager_C|GetActivePlayer _turnmanager) "/Game/AdvancedTurnBasedTileToolkit/Core/Abilities/BP_Ability_EnemyDisplay.BP_Ability_EnemyDisplay_C" self))))

(event EventTick
  (params (DeltaSeconds :type Float%20%28single-precision%29)))

(fn ConstructionScript
  (|CallParentFunction))
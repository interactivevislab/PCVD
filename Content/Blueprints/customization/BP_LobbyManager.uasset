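; Lobby manager that runs the menu flow and soldier squad customization, switching cameras and widgets through a state machine.
; Clicked spawn avatars open customization, where weapon, attachment and gene edits update PersonsInfo, with weapon and gene prices tallied in PowerSpend without enforcing the budget.
; Squad slots persist in a BP_SaveSquade save; choosing one replays its loadout onto the avatars, then saves and copies it to the GameInstance.
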(event Custom|ShowCustomizationWidgetForPerson
  (params (ID :type Integer))
  (bind _personsinfo (Variables|Default|GetpersonsInfo))
  (bind _output (Utilities|Array|Get(acopy) _personsinfo ID))
  (Viewport|RemoveAllWidgets)
  (Utilities|UIOnlyMode)
  (Game|Player|SetViewTargetwithBlend (Game|GetPlayerController 0) (Utilities|GetPersonCamera ID) (Variables|config|GetblendTimeToPerson) "VTBlend_Linear" 0.0 false)
  (Utilities|IsValid (Variables|Private|GetcustomizationWidget)
    (:Is%20Valid
      (Default|CallUpdateWidget _output ID))
    (:Is%20Not%20Valid
      (Widgets|CreateCustomizationWidget)
      (Default|ShowWidgetforSoldier (Variables|Private|GetcustomizationWidget) _output ID))))

(event Custom|HideCustomizationWidget
  (Widget|RemovefromParent (Variables|Private|GetcustomizationWidget))
  (Variables|Private|SetcustomizationWidget 0)
  (CallFunction|ChangeState "NewEnumerator4"))

(event Custom|MoveManagerCamera
  (params (Camera :type Camera%20Actor%20Object%20Reference))
  (Game|Player|SetViewTargetwithBlend (Game|GetPlayerController 0) Camera 1.0 "VTBlend_Linear" 0.0 false))

(event EventBeginPlay
  (CallFunction|ChangeState "NewEnumerator0")
  (init|InitPersonsArray)
  (Init|InitGenesInfoArray)
  (Load/Save|LoadSquad))

(event Collision|EventActorBeginOverlap
  (params (OtherActor :type Actor%20Object%20Reference)))

(event EventTick
  (params (DeltaSeconds :type Float%20%28single-precision%29)))

(fn ConstructionScript)

(fn InitPersonsArray
  (bind _outactors (Actor|GetAllActorsOfClass "/Game/Blueprints/units/BP_Unit_Avatar_Spawn.BP_Unit_Avatar_Spawn_C"))
  (for _array_element _outactors
    (Utilities|Array|SetArrayElem (Variables|Private|GetPersons) (Variables|/Game/Blueprints/units/BP_Unit_Avatar_Spawn.BP_Unit_Avatar_Spawn_C|Getid _array_element) _array_element true)
    (EventDispatchers|BindEventtoClickedonThisSoldier _array_element (EventDispatchers|CreateEvent :!event ShowCustomizationWidgetforPerson))
    (Default|ChangeWeapon _array_element (CallFunction|GetDefaultWeapon))))

(fn InitArrayPersonInfo
  (Utilities|Array|Clear (Variables|Default|GetpersonsInfo))
  (bind _mesh (CallFunction|GetUserMesh))
  (for _array_element (Variables|Private|GetPersons)
    (Utilities|Array|Add (Variables|Default|GetpersonsInfo) (Utilities|Struct|MakeST_Soldier 0 (CallFunction|GetDefaultWeapon) _mesh "(Type_6_CDDE11A9464D4E526B9B5AB61604554A=NewEnumerator0,Name_10_2550084D49B17AE608FBFEAB4A99BD3D=\"\",Icon_12_6D638F0B49BC101167EFB2915414ACE8=None,Mesh_16_EC2A6C6041ED3F286DEB4FA3898E24BA=None)" "(Type_6_CDDE11A9464D4E526B9B5AB61604554A=NewEnumerator0,Name_10_2550084D49B17AE608FBFEAB4A99BD3D=\"\",Icon_12_6D638F0B49BC101167EFB2915414ACE8=None,Mesh_16_EC2A6C6041ED3F286DEB4FA3898E24BA=None)" 0 0 0 0 0))
    (Utilities|IsValid _mesh
      (:Is%20Valid
        (Class|SkinnedMeshComponent|SetSkeletalMesh (Variables|/Game/Blueprints/units/BP_Unit_Anim_Avatar.BP_Unit_Anim_Avatar_C|GetMesh _array_element) _mesh true)))))

(fn InitGenesInfoArray
  (bind _outrownames (DataTable|GetDataTableRowNames "/Game/Blueprints/core/dataTable/DT_Genes.DT_Genes"))
  (for _array_element _outrownames
    (bind _returnvalue (Utilities|GetDataTableRow "/Game/Blueprints/core/dataTable/DT_Genes.DT_Genes" _array_element)
      (:then
        (Utilities|Map|Add (Variables|Private|GetgenesInfoMAp) (.GeneType (Utilities|Struct|BreakST_Genes_BP _returnvalue)) _returnvalue)))))

(fn GetUserPower
  (return (Variables|private|GetPower)))

(fn RequestUserPowerTransaction
  (params (changeValue :type Integer))
  (Utilities|CheckOpportunitytoSpendPower changeValue
    (:validTransaction
      _)
    (:invalidTransaction
      _))
  (Variables|Private|SetpowerSpend (+ (Variables|Private|GetpowerSpend) changeValue))
  (return true))

(fn CreateCustomizationWidget
  (bind _returnvalue (UserInterface|CreateWidget "/Game/Blueprints/UI/customization/WBP_CustomPerson.WBP_CustomPerson_C"))
  (Default|SetCustomizationManager _returnvalue self)
  (UserInterface|Viewport|AddtoViewport _returnvalue 0)
  (Variables|Private|SetcustomizationWidget _returnvalue))

(fn ChangeGenCountforPerson
  (params (ID :type Integer) (GenType :type E_GeneType%20Enum :default "NewEnumerator4") (changeValue :type Integer))
  (bind _returnvalue (Math|Integer|Absolute(Integer) changeValue))
  (bind _newparam (CallFunction|GetGenPrice GenType))
  (bind _returnvalue_2 (* _newparam _returnvalue))
  (LocalVariables|SetsoldierInfo (Utilities|Array|Get(acopy) (Variables|Default|GetpersonsInfo) ID))
  (if (> changeValue 0)
    (CallFunction|RequestUserPowerTransaction (* _returnvalue_2 -1))
    (else
      (CallFunction|RequestUserPowerTransaction _returnvalue_2)))
  (switch Utilities|FlowControl|Switch|SwitchonE_GeneType GenType
    (:NewEnumerator4
      (LocalVariables|SetcurentGenValue (.skeletalsystem_genvalue (LocalVariables|GetsoldierInfo)))
      (bind _structout (Utilities|Struct|SetmembersinST_Soldier (LocalVariables|GetsoldierInfo) (+ (LocalVariables|GetcurentGenValue) changeValue)))
      (LocalVariables|SetsoldierInfo _structout))
    (:NewEnumerator0
      (LocalVariables|SetcurentGenValue (.muscularsystem_genvalue (LocalVariables|GetsoldierInfo)))
      (bind _structout_2 (Utilities|Struct|SetmembersinST_Soldier (LocalVariables|GetsoldierInfo) (+ (LocalVariables|GetcurentGenValue) changeValue)))
      (LocalVariables|SetsoldierInfo _structout_2))
    (:NewEnumerator1
      (LocalVariables|SetcurentGenValue (.eyesystem_genvalue (LocalVariables|GetsoldierInfo)))
      (bind _structout_3 (Utilities|Struct|SetmembersinST_Soldier (LocalVariables|GetsoldierInfo) (+ (LocalVariables|GetcurentGenValue) changeValue)))
      (LocalVariables|SetsoldierInfo _structout_3))
    (:NewEnumerator2
      (LocalVariables|SetcurentGenValue (.nervoussystem_genvalue (LocalVariables|GetsoldierInfo)))
      (bind _structout_4 (Utilities|Struct|SetmembersinST_Soldier (LocalVariables|GetsoldierInfo) (+ (LocalVariables|GetcurentGenValue) changeValue)))
      (LocalVariables|SetsoldierInfo _structout_4)))
  (Utilities|Array|SetArrayElem (Variables|Default|GetpersonsInfo) ID (LocalVariables|GetsoldierInfo))
  (Default|CallUpdateWidget (Utilities|Array|Get(acopy) (Variables|Default|GetpersonsInfo) ID) ID))

(fn GetGenPrice
  (params (GenType :type E_GeneType%20Enum :default "NewEnumerator4"))
  (return (.Price (Utilities|Struct|BreakST_Genes_BP (.Value (Utilities|Map|Find (Variables|Private|GetgenesInfoMAp) GenType))))))

(fn ChangeWeaponforPerson
  (params (NewParam :type ST%20Weapon%20Structure) (id :type Integer))
  (CallFunction|RequestUserPowerTransaction (.Price (Utilities|Struct|BreakST_Weapon (.Weapon (Utilities|Struct|BreakST_Soldier (Utilities|Array|Get(acopy) (Variables|Default|GetpersonsInfo) id))))))
  (bind _successtransaction_ (CallFunction|RequestUserPowerTransaction (* (.Price (Utilities|Struct|BreakST_Weapon NewParam)) -1)))
  (if _successtransaction_
    (bind _structout (Utilities|Struct|SetmembersinST_Soldier (Utilities|Array|Get(acopy) (Variables|Default|GetpersonsInfo) id) NewParam))
    (Utilities|Array|SetArrayElem (Variables|Default|GetpersonsInfo) id _structout true)
    (Default|ChangeWeapon (Utilities|Array|Get(acopy) (Variables|Private|GetPersons) id) NewParam)
    (Default|CallUpdateWidget (Utilities|Array|Get(acopy) (Variables|Default|GetpersonsInfo) id) id)))

(fn FindGamesState
  (Viewport|RemoveAllWidgets)
  (if (Variables|Default|GetuseDedicatedServer)
    (bind _asgi_avatar_game_instance (Utilities|Casting|CastToGI_AvatarGameInstance (Game|GetGameInstance)))
    (Default|ConnecttoDedicatedServer _asgi_avatar_game_instance (Utilities|String|StringToName (Variables|Default|GetserverIP)))
    (Utilities|UIGameMode)
    (else
      (bind _returnvalue (UserInterface|CreateWidget "/Game/Blueprints/MainMenu.MainMenu_C" (Game|GetPlayerController 0) self))
      (UserInterface|Viewport|AddtoViewport _returnvalue 0)
      (Utilities|UIGameMode))))

(fn ChangeState
  (params (NewState :type E_LobbyState%20Enum :default "NewEnumerator0"))
  (bind _output_get (Variables|States|SetCurrentState NewState))
  (switch Utilities|FlowControl|Switch|SwitchonE_LobbyState _output_get
    (:NewEnumerator0
      (States|MainMenuState))
    (:NewEnumerator1
      (States|CreateGameState))
    (:NewEnumerator2
      (States|FindGamesState))
    (:NewEnumerator4
      (States|SquadOverviewState))
    (:NewEnumerator3
      (States|SetupSquadState))
    (:NewEnumerator5
      (States|AvatarCustomizationState))
    (:NewEnumerator6
      (States|ExitGameState))
    (:NewEnumerator7
      (States|LogOutState))))

(fn MainMenuState
  (Viewport|RemoveAllWidgets)
  (CallFunction|MoveManagerCamera (Variables|Default|GetMainMenuCamera))
  (bind _returnvalue (UserInterface|CreateWidget "/Game/Blueprints/UI/WBP_Lobby.WBP_Lobby_C" (Game|GetPlayerController 0) self))
  (bind _userinfo (CallFunction|GetUserInfo))
  (Default|SetUserInfo _returnvalue _userinfo)
  (UserInterface|Viewport|AddtoViewport _returnvalue 0)
  (Utilities|UIOnlyMode)
  (bind _userinfo_2 (CallFunction|GetUserInfo))
  (Variables|private|SetPower (.game_power _userinfo_2))
  (EventDispatchers|BindEventtoChoseSlot (Variables|/Game/Blueprints/UI/WBP_Lobby.WBP_Lobby_C|GetWBP_SlotSquads _returnvalue) (EventDispatchers|CreateEvent :!event ChoseSlot)))

(fn CreateGameState
  (Utilities|UIGameMode)
  (bind _asgi_avatar_game_instance (Utilities|Casting|CastToGI_AvatarGameInstance (Game|GetGameInstance)))
  (Default|StartSession _asgi_avatar_game_instance))

(fn SetupSquadState)

(fn AvatarCustomizationState
  (Viewport|RemoveAllWidgets)
  (CallFunction|MoveManagerCamera (Variables|Default|GetCustomizationCamera)))

(fn ExitGameState
  (Game|QuitGame 0 "Quit" false))

(fn SquadOverviewState
  (Viewport|RemoveAllWidgets)
  (CallFunction|MoveManagerCamera (Variables|Default|GetOverviewCamera))
  (bind _returnvalue (UserInterface|CreateWidget "/Game/Blueprints/UI/WBP_TeamView.WBP_TeamView_C" 0 self))
  (bind _userinfo (CallFunction|GetUserInfo))
  (Default|SetUserInfoTeamView _returnvalue _userinfo)
  (UserInterface|Viewport|AddtoViewport _returnvalue 0)
  (Utilities|UIGameMode))

(fn SaveSquadState
  (bind _loadsquadslot (Variables|Default|GetLoadSquadSlot))
  (bind _asgi_avatar_game_instance (Utilities|Casting|CastToGI_AvatarGameInstance (Game|GetGameInstance)))
  (bind _output_get (Variables|/Game/Blueprints/core/GI_AvatarGameInstance.GI_AvatarGameInstance_C|SetChoisenSoldiers _asgi_avatar_game_instance (Variables|Default|GetpersonsInfo)))
  (Default|SetSaveSquadSLot _loadsquadslot _output_get (Variables|Default|GetcurentActiveSlot))
  (SaveGame|SaveGametoSlot _loadsquadslot "SaveSquad")
  (Development|PrintString "Game Squad Save"))

(fn LogOutState
  (Class|AvatarApiManager|UserExit (CallFunction|GetApiManager))
  (Game|OpenLevel(byName) "AuthorizationLevel"))

(fn SetAttachmentsforPerson
  (params (Attachments :type ST%20Clothes%20Structure) (id :type Integer))
  (bind _personsinfo (Variables|Default|GetpersonsInfo))
  (bind _output (Utilities|Array|Get(acopy) _personsinfo id))
  (switch Utilities|FlowControl|Switch|SwitchonE_Clothes (.Type (Utilities|Struct|BreakST_Clothes Attachments))
    (:NewEnumerator0
      (bind _structout (Utilities|Struct|SetmembersinST_Soldier _output Attachments))
      (Utilities|Array|SetArrayElem (Variables|Default|GetpersonsInfo) id _structout))
    (:NewEnumerator1
      (bind _structout_2 (Utilities|Struct|SetmembersinST_Soldier _output Attachments))
      (Utilities|Array|SetArrayElem (Variables|Default|GetpersonsInfo) id _structout_2)))
  (Default|SetAttachment (Utilities|Array|Get(acopy) (Variables|Private|GetPersons) id) Attachments))

(fn GetDefaultWeapon
  (bind _returnvalue (Utilities|GetDataTableRow "/Game/Blueprints/core/dataTable/DT_Weapons.DT_Weapons" "Empty")
    (:then
      (return _returnvalue))))

(fn GetSpentPower
  (return (Variables|Private|GetpowerSpend)))

(fn SetEnableforSaveSquad
  (params (HavePower :type Boolean))
  ;[1 0.9839 0] CheckCanSaveSquad
  (Variables|Default|SetCanSaveSquad%28HaveMoney?%29 HavePower))

(fn LoadSquad
  (bind _returnvalue (SaveGame|DoesSaveGameExist "SaveSquad"))
  (if _returnvalue
    (bind _returnvalue_2 (SaveGame|LoadGamefromSlot "SaveSquad"))
    (bind _asbp_save_squade (Utilities|Casting|CastToBP_SaveSquade _returnvalue_2))
    (Variables|Default|SetLoadSquadSlot _asbp_save_squade)
    (Development|PrintString "GameLoaded" true true "(R=1.000000,G=0.000000,B=0.015526,A=1.000000)")
    (else
      (Development|PrintString "No Save Data" true true "(R=1.000000,G=0.000000,B=0.022868,A=1.000000)")
      (bind _returnvalue_3 (SaveGame|CreateSaveGameObject "/Game/Blueprints/core/BP_SaveSquade.BP_SaveSquade_C"))
      (Variables|Default|SetLoadSquadSlot _returnvalue_3)))
  (Load/Save|ChoseSlot 1))

(fn ShowSquadSlot
  (params (slotInfo :type Array%20of%20ST%20Soldier%20Structures))
  (CallFunction|ResetUserPowerSpent)
  (for (_array_element _array_index) slotInfo
    (Load/Save|SetUnit _array_element _array_index)))

(fn ChoseSlot
  (params (slot :type Integer))
  (bind _loadsquadslot (Variables|Default|GetLoadSquadSlot))
  (bind _output (Default|GetSquadSlot _loadsquadslot slot))
  (Init|InitArrayPersonInfo)
  (bind _output_get (Variables|Default|SetcurentActiveSlot slot))
  (if (Default|CheckSlotExist (Variables|Default|GetLoadSquadSlot) _output_get)
    (switch int _output_get
      (:1
        (Load/Save|ShowSquadSlot _output))
      (:2
        (Load/Save|ShowSquadSlot _output))
      (:3
        (Load/Save|ShowSquadSlot _output)))
    (else
      ;[1 1 1] show default Squad
      (Load/Save|ShowSquadSlot (Variables|Default|GetpersonsInfo))))
  (Load/Save|SaveSquadState))

(fn InitSquadSlotWidget)

(fn SetUnit
  (params (soldierInfo :type ST%20Soldier%20Structure) (id :type Integer))
  (bind (_price _weapon _bodymesh _headattachment) (Utilities|Struct|BreakST_Soldier soldierInfo))
  (CallFunction|ChangeWeaponforPerson _weapon id)
  (CallFunction|SetAttachmentsforPerson _headattachment id)
  (bind _mesh (CallFunction|GetUserMesh))
  (Default|SetMesh (Utilities|Array|Get(acopy) (Variables|Private|GetPersons) id) _mesh)
  (CallFunction|ChangeGenCountforPerson id "NewEnumerator4" (.skeletalsystem_genvalue soldierInfo))
  (CallFunction|ChangeGenCountforPerson id "NewEnumerator0" (.muscularsystem_genvalue soldierInfo))
  (CallFunction|ChangeGenCountforPerson id "NewEnumerator1" (.eyesystem_genvalue soldierInfo))
  (CallFunction|ChangeGenCountforPerson id "NewEnumerator2" (.nervoussystem_genvalue soldierInfo)))

(fn ResetUserPowerSpent
  (Variables|Private|SetpowerSpend 0))
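; BP_ActorRoom is an AR room actor that turns the static meshes of its Stol object into real-world occluders.
; On BeginPlay it gives each mesh a dynamic ARCore occlusion material, or a passthrough camera material on non-AR platforms.
; Tick updates the occlusion instances on AR platforms.
; ChangeMaterial swaps in an opaque material for edit mode, and SetAltRootToWorldZero shifts the actor so AltRoot lands on world origin.
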(event Custom|UpdateMaterial)

(event EventBeginPlay
  (Utilities|Array|Clear (Variables|Default|GetStaticMeshes))
  (for _array_element (Actor|GetComponentsByClass (Variables|Default|Getstol) "/Script/Engine.StaticMeshComponent")
    (Utilities|Array|Add (Variables|Default|GetStaticMeshes) _array_element)
    (Utilities|IsARSupportedPlatform
      (:true
        (Development|PrintString (Utilities|String|Append "CreateOcludsionMat for             " (Utilities|GetDisplayName _array_element)) true true "(R=0.000000,G=0.660000,B=1.000000,A=1.000000)" 1e+01)
        (bind _returnvalue (Rendering|Material|CreateDynamicMaterialInstance _array_element 0 "/Game/Materials/ARCoreOcclusionMaterial_001.ARCoreOcclusionMaterial_001" "None" :!class /Script/Engine.PrimitiveComponent))
        (bind _returnvalue_2 (Utilities|Array|Add (Variables|Default|GetMatInstances) _returnvalue))
        (Rendering|Material|SetMaterial (Utilities|Array|Get(acopy) (Variables|Default|GetStaticMeshes) _returnvalue_2) 0 _returnvalue))
      (:false
        (bind _returnvalue_3 (Rendering|Material|CreateDynamicMaterialInstance _array_element 0 "/Game/Materials/ExternalCamera/M_PassthroughCamera.M_PassthroughCamera" "None" :!class /Script/Engine.PrimitiveComponent))
        (bind _returnvalue_4 (Utilities|Array|Add (Variables|Default|GetMatInstances) _returnvalue_3))
        (Rendering|Material|SetMaterial (Utilities|Array|Get(acopy) (Variables|Default|GetStaticMeshes) _returnvalue_4) 0 _returnvalue_3)))))

(event Collision|EventActorBeginOverlap
  (params (OtherActor :type Actor%20Object%20Reference)))

(event EventTick
  (params (DeltaSeconds :type Float%20%28single-precision%29))
  (Utilities|IsARSupportedPlatform
    (:true
      (for _array_element (Variables|Default|GetMatInstances)
        ;[1 1 1] Occluder logic
        (CallFunction|UpdateARCoreOcclusionMaterialInstance _array_element)))))

(fn ConstructionScript)

(fn ChangeMaterial
  (params (EditMode :type Boolean))
  (for (_array_element _array_index) (Variables|Default|GetStaticMeshes)
    (Rendering|Material|SetMaterial _array_element 0 (select EditMode "/Game/Materials/BasicOpaqmaterial.BasicOpaqmaterial" (Utilities|Array|Get(acopy) (Variables|Default|GetMatInstances) _array_index)))))

(fn SetAltRoottoWorldZero
  (Transformation|SetActorLocation (- (Transformation|GetActorLocation) (Transformation|GetWorldLocation (Variables|Default|GetAltRoot))) false false))
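; PC spectator pawn that follows an Alt tracker to mirror its tracked pose.
; BeginPlay takes AltRoot from BP_ActorRoom and enables tick, which passes the tracker pose through AltCorection and adds MagicLocationFix and MagicRotationFix offsets.
; F and H draw and print tracker forward rays from fixed origins for calibration debugging.
; Hardcoded transform tests, input enabling and media plate assignment are left unwired.
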(event Custom|1111
  (bind _returnvalue (Math|Vector|MakeVector 0.0 -0.892 0.451))
  (bind _returnvalue_2 (Math|Vector|MakeVector 0.0 0.856 -0.515))
  (bind _returnvalue_3 (Math|Vector|VectorUp))
  (bind _returnvalue_4 (Math|Vector|VectorUp))
  (bind _returnvalue_5 (Math|Vector|Normalize _returnvalue_2))
  (bind _returnvalue_6 (* _returnvalue_3 _returnvalue))
  (bind _returnvalue_7 (Math|Vector|CrossProduct _returnvalue_4 _returnvalue_5))
  (bind _returnvalue_8 (Math|Vector|Normalize _returnvalue_7))
  (Development|PrintString (Utilities|String|ToString(Vector) (Math|Transform|InverseTransformLocation (Math|Transform|MakeTransform "5.851000,-164.481995,92.634003" (Math|Rotator|MakeRotationfromAxes _returnvalue_5 _returnvalue_8 (Math|Vector|Normalize (Math|Vector|CrossProduct _returnvalue_5 _returnvalue_8)))) "0.000000,-184.276993,110.867996")) true true "(R=0.107145,G=1.000000,B=0.000000,A=1.000000)" 1e+03)
  (Development|PrintString (Utilities|String|ToString(Vector) (Math|Transform|InverseTransformLocation (Utilities|NewMacro0 _returnvalue_6 (* _returnvalue_6 _returnvalue) _returnvalue "5.880000,-164.701004,94.134003") "0,-184.276993,110.867996")) true true "(R=1.000000,G=0.000000,B=0.052035,A=1.000000)" 1e+03))

(event EventBeginPlay
  (bind _returnvalue (Actor|GetActorOfClass "/Game/Blueprints/BP_ActorRoom.BP_ActorRoom_C"))
  (Utilities|IsValid _returnvalue
    (:Is%20Valid
      (Variables|Default|SetAltRoot (Variables|/Game/Blueprints/BP_ActorRoom.BP_ActorRoom_C|GetAltRoot _returnvalue))
      (bind _returnvalue_2 (Actor|GetActorOfClass "/Composure/Blueprints/CompositingElements/BP_MediaPlateCompElement.BP_MediaPlateCompElement_C"))
      (Actor|Tick|SetActorTickEnabled true))))

(event Collision|EventActorBeginOverlap
  (params (OtherActor :type Actor%20Object%20Reference)))

(event EventTick
  (params (DeltaSeconds :type Float%20%28single-precision%29))
  (bind _bp_alttracker (Variables|Default|GetBP_AltTracker))
  (bind _trackingtransform (Variables|/AntilatencyTracking/Blueprints/Samples/SceneComponents/BP_AltTracker.BP_AltTracker_C|GetTrackingTransform _bp_alttracker))
  (bind (_outlocation _outrotation) (Utilities|AltCorection (.location _trackingtransform) (.rotation _trackingtransform)))
  (Transformation|SetActorTransform (Math|Transform|MakeTransform (+ (Variables|Default|GetMagicLocationFix) _outlocation) (Math|Rotator|CombineRotators _outrotation (Variables|Default|GetMagicRotationFix)) "1,1,1")))

(event Input|KeyboardEvents|F
  (params (Key :type Key%20Structure :default "None"))
  (bind _bp_alttracker (Variables|Default|GetBP_AltTracker))
  (bind _bp_alttracker_2 (Variables|Default|GetBP_AltTracker))
  (bind _returnvalue (Math|Vector|GetForwardVector _bp_alttracker))
  (bind _returnvalue_2 (Transformation|GetWorldLocation _bp_alttracker_2))
  (bind _returnvalue_3 (Math|Vector|GetForwardVector _bp_alttracker_2))
  (bind _returnvalue_4 (* _returnvalue -1))
  (bind _returnvalue_5 (* _returnvalue_3 5e+02))
  (:Pressed
    (Variables|Default|SetstartLocation "0.000000,35.000000, 0")
    (Rendering|Debug|DrawDebugLine (Variables|Default|GetstartLocation) (+ (* _returnvalue_4 100000) (Variables|Default|GetstartLocation)) "(R=1.000000,G=0.000000,B=0.021617,A=1.000000)" 1e+03 0.5)
    (Rendering|Debug|DrawDebugLine (- _returnvalue_2 _returnvalue_5) (+ _returnvalue_2 _returnvalue_5) "(R=1.000000,G=0.833344,B=0.000000,A=1.000000)" 1e+03 0.5)
    (Development|PrintString (Utilities|String|Append "0   35    altForward   =====   " (Utilities|String|ToString(Vector) _returnvalue_4) "         alt Location      =====   " (Utilities|String|ToString(Vector) _returnvalue_2)))))

(event Input|KeyboardEvents|H
  (params (Key :type Key%20Structure :default "None"))
  (bind _bp_alttracker (Variables|Default|GetBP_AltTracker))
  (bind _bp_alttracker_2 (Variables|Default|GetBP_AltTracker))
  (bind _returnvalue (Math|Vector|GetForwardVector _bp_alttracker))
  (bind _returnvalue_2 (Transformation|GetWorldLocation _bp_alttracker_2))
  (bind _returnvalue_3 (Math|Vector|GetForwardVector _bp_alttracker_2))
  (bind _returnvalue_4 (* _returnvalue -1))
  (bind _returnvalue_5 (* _returnvalue_3 5e+02))
  (:Pressed
    (Variables|Default|SetstartLocation "0.000000,0.000000,0.000000")
    (Rendering|Debug|DrawDebugLine (Variables|Default|GetstartLocation) (+ (* _returnvalue_4 100000) (Variables|Default|GetstartLocation)) "(R=1.000000,G=0.000000,B=0.021617,A=1.000000)" 1e+03 0.5)
    (Rendering|Debug|DrawDebugLine (- _returnvalue_2 _returnvalue_5) (+ _returnvalue_2 _returnvalue_5) "(R=1.000000,G=0.833344,B=0.000000,A=1.000000)" 1e+03 0.5)
    (Development|PrintString (Utilities|String|Append "0    0      altForward   =====   " (Utilities|String|ToString(Vector) _returnvalue_4) "         alt Location      =====   " (Utilities|String|ToString(Vector) _returnvalue_2)))))

(fn ConstructionScript)

(fn NewFunction0
  (params (ForwardVectorAlt :type Vector) (AltPos :type Vector) (AltRot :type Rotator))
  (return (Math|Transform|InverseTransformLocation (Math|Transform|MakeTransform AltPos AltRot) (Transformation|GetWorldLocation (Variables|Default|GetCineCamera))) AltRot))
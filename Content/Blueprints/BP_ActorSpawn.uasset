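; BP_ActorSpawn is a line-trace test Blueprint that, despite its name, spawns nothing.
; A helper function returns the Sphere component's location and a point a fixed distance along its forward vector as trace endpoints.
; E runs a single object-type trace against world and physics objects, and F runs a multi trace on the Visibility channel.
; Both draw timed debug lines and leave their hit results unused.
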(event Input|KeyboardEvents|E
  (params (Key :type Key%20Structure :default "None"))
  (:Pressed
    (bind (_returnvalue _returnvalue2) (CallFunction|NewFunction0))
    (Collision|LineTraceForObjects _returnvalue _returnvalue2 (Utilities|Array|MakeArray "ObjectTypeQuery1" "ObjectTypeQuery2" "ObjectTypeQuery4") false 0 "ForDuration")))

(event Input|KeyboardEvents|F
  (params (Key :type Key%20Structure :default "None"))
  (:Pressed
    (bind (_returnvalue _returnvalue2) (CallFunction|NewFunction0))
    (Collision|MultiLineTraceByChannel _returnvalue _returnvalue2 "TraceTypeQuery1" false 0 "ForDuration")))

(fn ConstructionScript)

(fn NewFunction0
  (bind _sphere (Variables|Default|GetSphere))
  (bind _returnvalue (Transformation|GetWorldLocation _sphere))
  (return _returnvalue (+ _returnvalue (* (Math|Vector|GetForwardVector _sphere) 5e+02))))
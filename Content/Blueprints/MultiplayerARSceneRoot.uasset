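; Multiplayer AR scene root actor that aligns its CloudARPinRoot component to a cloud AR pin.
; On authority, it copies RoomID from the avatar game instance at BeginPlay and accepts CloudID updates.
; AttachToCloudARPin only stores the pin reference.
; Tick snaps CloudARPinRoot to the pin's world transform while the pin is tracking and CanMove is set, rather than using component attachment.
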(event EventBeginPlay
  (Networking|SwitchHasAuthority
    (:Authority
      (bind _asgi_avatar_game_instance (Utilities|Casting|CastToGI_AvatarGameInstance (Game|GetGameInstance)))
      (Variables|Default|SetRoomID (Variables|/Game/Blueprints/core/GI_AvatarGameInstance.GI_AvatarGameInstance_C|GetRoomID _asgi_avatar_game_instance)))))

(event EventTick
  (params (DeltaSeconds :type Float%20%28single-precision%29))
  (bind _cloudarpin (Variables|Default|GetCloudARPin))
  (Utilities|FlowControl|Sequence
    (:then_0
      (if (Utilities|IsValid (Variables|Default|GetCloudARPin))
        (if (Utilities|Enum|Equal(Enum) (Class|ARPin|GetTrackingState _cloudarpin) "Tracking")
          (if (Variables|Default|GetCanMove)
            (Transformation|SetWorldTransform (Variables|Default|GetCloudARPinRoot) (Class|ARPin|GetLocaltoWorldTransform _cloudarpin) false false)))))))

(fn ConstructionScript)

(fn SetCloudID
  (params (CloudID :type String))
  (Networking|SwitchHasAuthority
    (:Authority
      (Variables|Default|SetCloudID CloudID))))

(fn AttachtoCloudARPin
  (params (CloudARPin :type Cloud%20AR%20Pin%20Object%20Reference))
  (Variables|Default|SetCloudARPin CloudARPin))
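; BP_Unit_Avatar_Spawn is a soldier avatar that displays a unit's body, head attachment and weapon, and broadcasts its Id when its touch box is tapped.
; SetUnit applies the soldier info through ChangeWeapon, SetAttachment and UpdateMesh.
; ChangeWeapon shows either a skeletal or static weapon mesh, then AnimateWeaponReaction swaps the anim class by weapon type, with melee also playing a sword-and-shield idle montage.
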(event OnInputTouchBegin(BoxForTouch)
  (params (FingerIndex :type ETouchIndex%20Enum :default "Touch1") (TouchedComponent :type Primitive%20Component%20Object%20Reference))
  (Default|CallClickedonThisSoldier (Variables|CustomizationOnly|Getid)))

(event Custom|AnimateWeaponReaction
  (params (WeaponType :type E_WeaponType%20Enum :default "NewEnumerator0"))
  (bind _mesh (Variables|Character|GetMesh))
  (switch Utilities|FlowControl|Switch|SwitchonE_WeaponType WeaponType
    (:NewEnumerator0
      (Class|SkeletalMeshComponent|SetAnimClass _mesh "/Game/Animations/Dima/Retarget/ABP_Avatar_Dima_Meele.ABP_Avatar_Dima_Meele_C")
      (Animation|Montage|PlayMontage _mesh "/Game/Animations/Sword_And_Shield_Idle_Montage.Sword_And_Shield_Idle_Montage" 1.0 0.0 "Default"))
    (:NewEnumerator1
      (Class|SkeletalMeshComponent|SetAnimClass (Variables|Character|GetMesh) "/Game/Animations/Dima/Retarget/ABP_Avatar_Dima.ABP_Avatar_Dima_C" :!label _label))
    (:NewEnumerator2
      (goto _label))
    (:NewEnumerator3
      (goto _label))
    (:NewEnumerator4
      (goto _label))))

(event EventBeginPlay
  (|CallParentFunction))

(event Collision|EventActorBeginOverlap
  (params (OtherActor :type Actor%20Object%20Reference))
  (|CallParentFunction OtherActor) ; This node is disabled and will not be called.\nDrag off pins to build functionality.
)

(event EventTick
  (params (DeltaSeconds :type Float%20%28single-precision%29))
  (|CallParentFunction DeltaSeconds) ; This node is disabled and will not be called.\nDrag off pins to build functionality.
)

(fn ConstructionScript
  (|CallParentFunction))

(fn ChangeWeapon
  (params (NewWeapon :type ST%20Weapon%20Structure))
  (bind _sm_weapon (Variables|Default|GetSM_Weapon))
  (Utilities|IsValid (.mesh NewWeapon)
    (:Is%20Valid
      (Class|SkinnedMeshComponent|SetSkeletalMesh (Variables|Default|GetWeaponSkM_0) (.mesh NewWeapon) true)
      (Rendering|SetVisibility (Variables|Default|GetSM_Weapon) false false)
      (Rendering|SetVisibility (Variables|Default|GetWeaponSkM_0) true false))
    (:Is%20Not%20Valid
      (Rendering|SetVisibility _sm_weapon true false)
      (Components|StaticMesh|SetStaticMesh _sm_weapon (.staticmesh NewWeapon))
      (Development|PrintString (Utilities|GetDisplayName (.staticmesh NewWeapon)))
      (Rendering|SetVisibility (Variables|Default|GetWeaponSkM_0) false false)))
  (CallFunction|AnimateWeaponReaction (.type NewWeapon)))

(fn SetUnit
  (params (soldierInfo :type ST%20Soldier%20Structure))
  (bind (_price _weapon _bodymesh _headattachment) (Utilities|Struct|BreakST_Soldier soldierInfo))
  (CallFunction|ChangeWeapon _weapon)
  (CallFunction|SetAttachment _headattachment)
  (CallFunction|UpdateMesh _bodymesh))

(fn SetAttachment
  (params (Attachments :type ST%20Clothes%20Structure))
  (bind (_type _name _icon _mesh) (Utilities|Struct|BreakST_Clothes Attachments))
  (switch Utilities|FlowControl|Switch|SwitchonE_Clothes _type
    (:NewEnumerator0
      (Components|StaticMesh|SetStaticMesh (Variables|Default|GetHeadAttachments) _mesh))))

(fn UpdateMesh
  (params (NewParam :type Skeletal%20Mesh%20Object%20Reference))
  (Class|SkinnedMeshComponent|SetSkeletalMesh (Variables|Character|GetMesh) NewParam true))
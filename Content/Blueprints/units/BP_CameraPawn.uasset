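; Camera pawn that handles selecting an avatar soldier and opening the WBP_CustomPerson widget for it.
; On BeginPlay it indexes every BP_Unit_Avatar_Spawn by Id and binds to each one's click event.
; A click hides and disables collision on all other soldiers, then creates the widget or makes the existing one visible.
; On first creation, input switches to UI-only with the mouse locked.
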(event Custom|clickToSoldier
  (params (SelectedSoldier :type Integer))
  ;[1 1 1] Second
  (Development|PrintString (Utilities|String|ToString(Integer) SelectedSoldier))
  (CallFunction|Hide SelectedSoldier))

(event Custom|Hide
  (params (id :type Integer))
  ;[1 1 1] Third
  (for _array_element (Variables|Default|GetArrayOfSoldiers)
    (if (not (== id (Variables|/Game/Blueprints/units/BP_Unit_Avatar_Spawn.BP_Unit_Avatar_Spawn_C|Getid _array_element)))
      (Rendering|SetActorHiddenInGame _array_element true)
      (Collision|SetActorEnableCollision _array_element false)))
  (CallFunction|OpenWidget))

(event Custom|OpenWidget
  (bind _returnvalue (Game|GetPlayerController 0))
  ;[1 1 1] Comment
  (if (Variables|Default|GetWidgetCreated)
    (Widget|SetVisibility (stale _returnvalue_2) "Visible")
    (else
      (bind _returnvalue_2 (UserInterface|CreateWidget "/Game/Blueprints/UI/WBP_CustomPerson.WBP_CustomPerson_C" _returnvalue))
      (UserInterface|Viewport|AddtoViewport _returnvalue_2 0)
      (Input|SetInputModeUIOnly _returnvalue _returnvalue_2 "LockAlways")
      (Variables|Default|SetWidgetCreated true))))

(event EventBeginPlay
  ;[1 1 1] First
  (bind _outactors (Actor|GetAllActorsOfClass "/Game/Blueprints/units/BP_Unit_Avatar_Spawn.BP_Unit_Avatar_Spawn_C"))
  (for _array_element _outactors
    (Utilities|Array|SetArrayElem (Variables|Default|GetArrayOfSoldiers) (Variables|/Game/Blueprints/units/BP_Unit_Avatar_Spawn.BP_Unit_Avatar_Spawn_C|Getid _array_element) _array_element true)
    (EventDispatchers|BindEventtoClickedonThisSoldier _array_element (EventDispatchers|CreateEvent :!event Custom|clickToSoldier))))

(fn ConstructionScript)
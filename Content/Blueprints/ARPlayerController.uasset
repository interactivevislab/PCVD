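; Player controller for multiplayer Cloud AR Pin sessions: creates pin and debug widgets locally and manages the ARCore session lifecycle.
; Tick finds the MultiplayerARSceneRoot, reports session errors, and on tracking-quality changes toggles the screensaver and pin-root visibility.
; ServerAddGameActor spawns actors offset from the shared pin root's transform, without attaching them.
; Android Back destroys the online session and opens the main menu.
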(event Custom|ServerAddGameActor
  (params (ActorClass :type Actor%20Class%20Reference) (RelativeTransform :type Transform))
  (bind (_location _rotation) (Math|Transform|BreakTransform RelativeTransform))
  (bind _arsceneroot (Variables|Default|GetARSceneRoot))
  (bind _cloudarpinroot (Variables|/Game/Blueprints/MultiplayerARSceneRoot.MultiplayerARSceneRoot_C|GetCloudARPinRoot _arsceneroot))
  ;[1 1 1] On server, spawn the game actor and attach it to ARSceneRoot actor using the relative transform passed in
  (bind _returnvalue (Game|SpawnActorfromClass ActorClass (Math|Transform|MakeTransform (+ _location (Transformation|GetWorldLocation _cloudarpinroot)) (Math|Rotator|CombineRotators _rotation (Transformation|GetWorldRotation _cloudarpinroot)) "1,1,1") "AlwaysSpawn" 0 0)))

(event EventBeginPlay
  ;[1 1 1] Create UIWidget for local player
  (if (Pawn|IsLocalPlayerController)
    (bind _returnvalue (UserInterface|CreateWidget "/Game/Blueprints/CloudARPinWidget.CloudARPinWidget_C" self))
    (bind _output_get (Variables|Default|SetCloudARPinWidget _returnvalue))
    (UserInterface|Viewport|AddtoViewport _output_get 0)
    ;[0.5506 0 1] Adding Debug Widget
    (bind _returnvalue_2 (UserInterface|CreateWidget "/Game/HandheldARBP/Blueprints/UI/BP_DebugMenu.BP_DebugMenu_C" (Game|GetPlayerController 0)))
    (bind _output_get_2 (Variables|Default|SetDebugMenuWidget _returnvalue_2))
    (UserInterface|Viewport|AddtoViewport _output_get_2 0)
    ;[1 1 1] Enable GoogleARCore Services and start ARSession
    (Utilities|IsARSupportedPlatform
      (:true
        (Class|GoogleARCoreServicesFunctionLibrary|ConfigGoogleARCoreServices (Utilities|Struct|MakeGoogleARCoreServicesConfig "Enabled"))
        (Class|ARBlueprintLibrary|StartARSession "/Game/Blueprints/CloudARPinSessionConfig.CloudARPinSessionConfig")
        (CallFunction|UpdateScreensaver)))))

(event EventTick
  (params (DeltaSeconds :type Float%20%28single-precision%29))
  (bind _returnvalue (Class|ARBlueprintLibrary|GetTrackingQuality))
  (bind _returnvalue_2 (Class|ARBlueprintLibrary|GetARSessionStatus))
  (Utilities|FlowControl|Sequence
    (:then_0
      ;[1 1 1] Get the ARSceneRoot Actor reference when it is spawned by the server
      (Utilities|IsValid (Variables|Default|GetARSceneRoot)
        (:Is%20Not%20Valid
          (bind _outactors (Actor|GetAllActorsOfClass "/Game/Blueprints/MultiplayerARSceneRoot.MultiplayerARSceneRoot_C"))
          (if (> (Utilities|Array|Length _outactors) 0)
            (Variables|Default|SetARSceneRoot (Utilities|Array|Get(acopy) _outactors))))))
    (:then_1
      ;[1 1 1] Show error when ARSession failed to start
      (switch Utilities|FlowControl|Switch|SwitchonEARSessionStatus (.status _returnvalue_2)
        (:Running
          (Utilities|FlowControl|Sequence
            (:then_0
              (if (!= (Variables|Default|GetPreviousTrackingQuality) _returnvalue)
                (CallFunction|UpdateScreensaver)
                (CallFunction|UpdateSceneActorVisibility)))
            (:then_1
              (Variables|Default|SetPreviousTrackingQuality _returnvalue))))
        (:NotSupported
          (Default|SetSnackbarOutput (Variables|Default|GetCloudARPinWidget) (Utilities|Text|ToText(String) (Utilities|Select :Index (.status _returnvalue_2) :NotStarted "" :Running "" :NotSupported "AR session failed to start becuase the device is not supported" :FatalError "AR session has unknown error." :PermissionNotGranted "Camera unavailable. Please restart the app." :UnsupportedConfiguration "" :Other "")) :!label _label))
        (:FatalError
          (goto _label))
        (:PermissionNotGranted
          (goto _label))))))

(event EventEndPlay
  (params (EndPlayReason :type EEndPlayReason%20Enum :default "Destroyed"))
  ;[1 1 1] Stop ARSession
  (if (Pawn|IsLocalPlayerController)
    (Class|ARBlueprintLibrary|StopARSession)))

(event Input|KeyboardEvents|AndroidBack
  (params (Key :type Key%20Structure :default "None"))
  (:Pressed
    ;[1 1 1] Return to main menu when Android back button is pressed
    (if (Pawn|IsLocalPlayerController)
      (|DestroySession self
        (:OnSuccess
          _)
        (:OnFailure
          _))
      (Game|OpenLevel(byName) "MainMenu"))))

(fn ConstructionScript)

(fn UpdateScreensaver
  (switch Utilities|FlowControl|Switch|SwitchonEARTrackingQuality (Class|ARBlueprintLibrary|GetTrackingQuality)
    (:NotTracking
      (if (not (Variables|Default|GetScreenSaverEnabled))
        (Class|KismetSystemLibrary|ControlScreensaver true)
        (Variables|Default|SetScreenSaverEnabled true)))
    (:OrientationAndPosition
      (if (Variables|Default|GetScreenSaverEnabled)
        (Class|KismetSystemLibrary|ControlScreensaver false)
        (Variables|Default|SetScreenSaverEnabled false)))))

(fn UpdateSceneActorVisibility
  (Rendering|SetVisibility (Variables|/Game/Blueprints/MultiplayerARSceneRoot.MultiplayerARSceneRoot_C|GetCloudARPinRoot (Variables|Default|GetARSceneRoot)) (Utilities|Select :Index (Class|ARBlueprintLibrary|GetTrackingQuality) :NotTracking false :OrientationOnly false :OrientationAndPosition true) true)
  (bind _returnvalue (Class|ARBlueprintLibrary|GetAllGeometries))
  (bind _array_element (Utilities|Array|ForEachLoopwithBreak _returnvalue)
    (:LoopBody
      (Class|ARBlueprintLibrary|DebugDrawTrackedGeometry _array_element "(R=1.000000,G=0.000000,B=0.478172,A=1.000000)"))))
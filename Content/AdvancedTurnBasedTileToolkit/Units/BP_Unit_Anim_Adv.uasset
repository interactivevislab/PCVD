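; BP_Unit_Anim_Adv is a unit Blueprint in the Advanced Turn Based Tile Toolkit that adds faction-based health bar coloring to its parent unit class.
; On BeginPlay it runs the parent logic, then checks whether the unit belongs to the first Faction enum value.
; For that faction, it creates a dynamic material instance on the HealthBar and sets its Color parameter to green.
; All other behavior, including construction, comes from the parent.
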(event EventBeginPlay
  (|CallParentFunction)
  (if (Utilities|Enum|Equal(Enum) (Variables|Default|GetFaction) "NewEnumerator0")
    (bind _returnvalue (Rendering|Material|CreateDynamicMaterialInstance (Variables|Default|GetHealthBar) 0 (Rendering|Material|GetMaterial (Variables|Default|GetHealthBar) 0) "None" :!class /Script/Engine.PrimitiveComponent))
    (Rendering|Material|SetVectorParameterValue _returnvalue "Color" "(R=0.000000,G=1.000000,B=0.000000,A=1.000000)" :!class /Script/Engine.MaterialInstanceDynamic)))

(event Collision|EventActorBeginOverlap
  (params (OtherActor :type Actor%20Object%20Reference)))

(event EventTick
  (params (DeltaSeconds :type Float%20%28single-precision%29)))

(fn ConstructionScript
  (|CallParentFunction))
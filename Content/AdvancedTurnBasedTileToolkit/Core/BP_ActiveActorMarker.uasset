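; BP_ActiveActorMarker is the tile-grid marker that highlights and follows the active unit.
; On BeginPlay it finds the grid manager and shows either a decal or a mesh, using the hex or square variant to match the grid.
; AnimateAction takes the unit from an action and scales the marker by tile and unit size, hiding it otherwise.
; Tick copies the followed unit's location and the grid's rotation and scale.
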(event EventTick
  (params (DeltaSeconds :type Float%20%28single-precision%29))
  (bind _gridmanagerref (Variables|Default|GetGridManagerRef))
  (bind _returnvalue (Transformation|GetActorTransform _gridmanagerref))
  (Utilities|IsValid (Variables|Default|GetActorToFollow)
    (:Is%20Valid
      (Transformation|SetActorTransform (Math|Transform|MakeTransform (Transformation|GetActorLocation (Variables|Default|GetActorToFollow)) (.rotation _returnvalue) (.scale _returnvalue))))))

(event EventAnimateAction
  (params (Action :type F%20Action%20Structure))
  (bind _gridmanagerref (Variables|Default|GetGridManagerRef))
  (switch name (CallFunction|GetActionName Action)
    (:FollowActor
      (bind _asbp_unit (Utilities|Casting|CastToBP_Unit (CallFunction|GetActor Action))
        (:then
          (Variables|Default|SetActorToFollow _asbp_unit)
          (Rendering|SetActorHiddenInGame false)
          (Transformation|SetWorldScale3D (Variables|Default|GetActiveActorMarkerMesh) (* (* (Transformation|GetActorScale3D _gridmanagerref) (/ (Variables|/Game/AdvancedTurnBasedTileToolkit/Core/Grid/BP_GridManager.BP_GridManager_C|GetTileXSize _gridmanagerref) 2e+02)) (Math|Conversions|ToFloat(Integer) (Math|Integer|Max(Integer) (Variables|/Game/AdvancedTurnBasedTileToolkit/Core/Units/BP_Unit.BP_Unit_C|GetSize _asbp_unit) 1)))))
        (:CastFailed
          (Rendering|SetActorHiddenInGame true))))))

(event EventBeginPlay
  (bind _outactors (Actor|GetAllActorsOfClass "/Game/AdvancedTurnBasedTileToolkit/Core/Grid/BP_GridManager.BP_GridManager_C"))
  (Variables|Default|SetGridManagerRef (Utilities|Array|Get(acopy) _outactors))
  (Variables|Default|SetbHexGrid (== (Utilities|GetClass (Utilities|Array|Get(acopy) _outactors)) "/Game/AdvancedTurnBasedTileToolkit/Core/Grid/BP_GridManager_Hex.BP_GridManager_Hex_C"))
  (if (Variables|/Game/AdvancedTurnBasedTileToolkit/Core/Grid/BP_GridManager.BP_GridManager_C|GetbUseDecals (Variables|Default|GetGridManagerRef))
    (Utilities|IsValid (select (Variables|Default|GetbHexGrid) (Variables|Default|GetActiveActorMarkerDecalHex) (Variables|Default|GetActiveActorMarkerDecalSquare))
      (:Is%20Valid
        (Rendering|Components|Decal|SetDecalMaterial (Variables|Default|GetActiveActorMarkerDecal) (select (Variables|Default|GetbHexGrid) (Variables|Default|GetActiveActorMarkerDecalHex) (Variables|Default|GetActiveActorMarkerDecalSquare))))
      (:Is%20Not%20Valid
        _))
    (Rendering|SetVisibility (Variables|Default|GetActiveActorMarkerDecal) true false)
    (else
      (Utilities|IsValid (select (Variables|Default|GetbHexGrid) (Variables|Default|GetActiveActorMarkerMeshHex) (Variables|Default|GetActiveActorMarkerMeshSquare))
        (:Is%20Valid
          (Components|StaticMesh|SetStaticMesh (Variables|Default|GetActiveActorMarkerMesh) (select (Variables|Default|GetbHexGrid) (Variables|Default|GetActiveActorMarkerMeshHex) (Variables|Default|GetActiveActorMarkerMeshSquare))))
        (:Is%20Not%20Valid
          _))
      (Rendering|SetVisibility (Variables|Default|GetActiveActorMarkerMesh) true false))))

(fn ConstructionScript)
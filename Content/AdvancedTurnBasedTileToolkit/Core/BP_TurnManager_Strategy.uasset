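; Strategy turn manager for the turn-based tile toolkit, running turns per faction rather than per actor.
; Faction turn start notifies its actors, waits on ongoing actions, then finds a refreshed actor: AI actors are auto-selected, otherwise queued actions play and player-owned factions get the idle ability.
; After each ability, unexhausted actors are reselected; exhausted AI passes to the next actor, while players return to idle until none remain or they end the turn.
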(event EventEndTurnfromPlayerInput
  ;[1 0.954 0] EndTurnFromPlayerInput
  (CallFunction|EndActiveFactionTurn))

(event EventBeginActiveFactionTurn
  ;[0 1 0.6948] Begin Active Faction Turn
  (bind _actorsoffaction (CallFunction|FindInitiativeActorsOfFaction (Variables|Default|GetActiveFaction)))
  (for _array_element _actorsoffaction
    (Class|BPIInitiative|RunonBeginActorTurn(Message) _array_element))
  (Class|BPIInitiative|DeselectActor(Message) (Variables|Default|GetActiveActor))
  (Utilities|WaitforOngoingActions)
  (bind (_bfoundvalidactor _actor) (CallFunction|FindNextRefreshedActor true (Variables|Default|GetActiveFaction)))
  (if _bfoundvalidactor
    (bind _asbp_player_controller_atbtt (Utilities|Casting|CastToBP_PlayerController_ATBTT (Components|GetOwner _actor))
      (:then
        (Variables|Default|SetActivePlayer _asbp_player_controller_atbtt)
        (Class|BPIAbility|ActivateAbility(Message) (Variables|Default|GetActivePlayer) "/Game/AdvancedTurnBasedTileToolkit/Core/Abilities/BP_AbilityBase_Idle.BP_AbilityBase_Idle_C" (Variables|Default|GetActivePlayer)))
      (:CastFailed
        (Variables|Default|SetActivePlayer 0)))
    (Utilities|QueueActionSingles self "DisplayFactionTurn" "NewEnumerator0" true -1 false 0.0 false 0 0.0 (Utilities|String|EnumtoString (Variables|Default|GetActiveFaction)))
    (bind _baicontrolled (Class|BPIInitiative|GetAiControlled(Message) _actor))
    (if _baicontrolled
      (Class|BPIInitiative|SelectActor(Message) _actor)
      (else
        (bind _actionmanager (Utilities|GetActionManager))
        (Default|InitializeQueuedActions _actionmanager)))
    (else
      (CallFunction|EndActiveFactionTurn))))

(event EventRunAfterAbilityExecute
  (bind _activeactor (Variables|Default|GetActiveActor))
  (bind _activeplayer (Variables|Default|GetActivePlayer))
  ;[0.4688 0 0.3991] Run After Ability Execute
  (bind _bexhausted (Class|BPIInitiative|CheckifExhausted(Message) (Variables|Default|GetActiveActor)))
  (if _bexhausted
    (bind _baicontrolled (Class|BPIInitiative|GetAiControlled(Message) _activeactor))
    (if _baicontrolled
      (CallFunction|BeginNextValidActorTurn)
      (else
        (bind _bfoundvalidactor (CallFunction|FindNextRefreshedActor true (Variables|Default|GetActiveFaction)))
        (if _bfoundvalidactor
          (Class|BPIAbility|ActivateAbility(Message) _activeplayer "/Game/AdvancedTurnBasedTileToolkit/Core/Abilities/BP_AbilityBase_Idle.BP_AbilityBase_Idle_C" _activeplayer)
          (bind _actionmanager (Utilities|GetActionManager))
          (Default|InitializeQueuedActions _actionmanager)
          (else
            (CallFunction|EndActiveFactionTurn)))))
    (else
      (Class|BPIInitiative|SelectActor(Message) _activeactor))))

(fn ConstructionScript
  (|CallParentFunction))
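; BP_GridCamera_Custom is a grid camera for the turn-based tile toolkit that overrides the camera Setup.
; Setup waits for the TurnManager, then places the camera at a unit from the initiative order, or at a point derived from grid bounds.
; Once PlayerState is valid, it notifies the server of readiness, then starts follow-cam ticking, edge scrolling, hover ticks and platform translucency handling.
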(event EventBeginPlay)

(event Collision|EventActorBeginOverlap
  (params (OtherActor :type Actor%20Object%20Reference)))

(event EventTick
  (params (DeltaSeconds :type Float%20%28single-precision%29)))

(event EventSetup
  ;[0 0.44 0.09101] Setup
  (bind _asbp_atbtt_state (Utilities|Casting|CastToBP_ATBTT_State (Game|GetGameState)))
  (Utilities|DelayWhile (not (Utilities|IsValid (Variables|/Game/AdvancedTurnBasedTileToolkit/Core/BP_ATBTT_State.BP_ATBTT_State_C|GetTurnManager _asbp_atbtt_state)))
    (:Continue
      (if (Utilities|IsValid (Utilities|Array|Get(acopy) (Variables|/Game/AdvancedTurnBasedTileToolkit/Core/BP_TurnManager.BP_TurnManager_C|GetInitiativeOrderActors (Variables|/Game/AdvancedTurnBasedTileToolkit/Core/BP_ATBTT_State.BP_ATBTT_State_C|GetTurnManager _asbp_atbtt_state)) 1))
        (Transformation|SetActorLocationAndRotation (Transformation|GetActorLocation (Utilities|Array|Get(acopy) (Variables|/Game/AdvancedTurnBasedTileToolkit/Core/BP_TurnManager.BP_TurnManager_C|GetInitiativeOrderActors (Variables|/Game/AdvancedTurnBasedTileToolkit/Core/BP_ATBTT_State.BP_ATBTT_State_C|GetTurnManager _asbp_atbtt_state)) 1)) "0, 0, 0")
        (else
          (bind _gridmanager (Utilities|GetGridManager))
          (Transformation|SetActorLocationAndRotation (/ (+ (.Origin (Collision|GetActorBounds _gridmanager false false)) (.BoxExtent (Collision|GetActorBounds _gridmanager false false))) 2.0) "0, 0, 0") ; If no units in initiative, center grid camera on grid
        ))
      (Utilities|DelayWhile (not (Utilities|IsValid (Variables|Default|GetPlayerState)))
        (:Continue
          (CallFunction|ServerNotifyPlayerReady)
          (Utilities|FlowControl|Delay 0.3)
          (CallFunction|UpdatePlatformTranslucency)
          (Actor|Tick|SetActorTickEnabled (Variables|Default|GetbUseFollowCam))
          (CallFunction|EdgeScrolling)
          (Class|BPIGridInteraction|ActivateHoverTick(Message) (Game|GetPlayerController 0))
          (bind _outactors (Actor|GetAllActorsOfClass "/Game/AdvancedTurnBasedTileToolkit/Core/Tiles/BP_GA_Platform.BP_GA_Platform_C"))
          (if (!= (Utilities|Array|Length _outactors) 0)
            (Variables|Default|SetbCheckPlatformTranslucency true)
            (CallFunction|HandlePlatformTranslucencyonFollow)))))))

(fn ConstructionScript
  (|CallParentFunction))
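; Turn manager for the hybrid map, switching play between real-time third-person exploration and grid-based turn combat.
; Entering combat snaps units to nearby free tiles, builds initiative from units in sight of the player, and blends to the grid camera.
; When one faction has no units left in initiative and the game is not over, it leaves turn-based mode and lerps back to possessing the third-person character.
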(event Custom|BeginTurnBasedMode
  (Default|CallOnTurnBasedBegin)
  (Utilities|Array|Clear (Variables|Default|GetInitiativeOrderActors))
  (bind _gridmanager (Utilities|GetGridManager))
  (bind _outactors (Actor|GetAllActorsOfClass "/Game/AdvancedTurnBasedTileToolkit/Maps/Experimental/Hybrid/BP_Unit_Hybrid.BP_Unit_Hybrid_C"))
  (for _array_element _outactors
    (bind _asbp_third_person_character (Utilities|Casting|CastToBP_ThirdPersonCharacter (Variables|/Script/Engine.ChildActorComponent|GetChildActor (Variables|/Game/AdvancedTurnBasedTileToolkit/Maps/Experimental/Hybrid/BP_Unit_Hybrid.BP_Unit_Hybrid_C|GetThirdPersonChild _array_element))))
    (bind (_bsuccess _tileindex) (Default|FindClosestValidEmptyTile _gridmanager (Transformation|GetWorldLocation (Variables|/Script/Engine.Character|GetCapsuleComponent _asbp_third_person_character)) 3))
    (if _bsuccess
      (Default|RemoveUnitfromGrid _gridmanager _array_element)
      (Default|AddUnittoGrid _gridmanager _array_element _tileindex true)
      (Transformation|SetActorLocation _array_element (- (Transformation|GetWorldLocation (Variables|/Script/Engine.Character|GetCapsuleComponent _asbp_third_person_character)) "0,0.000000,90.000000") false false)
      (Transformation|SetRelativeLocation (Variables|/Script/Engine.Actor|GetRootComponent _asbp_third_person_character) "0, 0, 0" false false)))
  (bind _asbp_third_person_character_2 (Utilities|Casting|CastToBP_ThirdPersonCharacter (Game|Player|GetPlayerPawn 0)))
  (bind _newparam (CallFunction|FindUnitsinSightOfActor _asbp_third_person_character_2))
  (bind _sortedactors (CallFunction|SortActorsinInitiativeOrder _newparam))
  (Variables|Default|SetInitiativeOrderActors _sortedactors)
  (Transformation|SetActorLocation (Variables|Default|GetGridCameraRef) (Transformation|GetActorLocation) false false)
  (Pawn|Possess (Game|GetPlayerController 0) (Variables|Default|GetGridCameraRef))
  (Default|LerpfromThirdPerson (Variables|Default|GetGridCameraRef) (Transformation|GetWorldTransform (Variables|/Game/AdvancedTurnBasedTileToolkit/Maps/Experimental/Hybrid/BP_ThirdPersonCharacter.BP_ThirdPersonCharacter_C|GetFollowCamera _asbp_third_person_character_2)) (Variables|/Script/Engine.CameraComponent|GetFieldOfView (Variables|/Game/AdvancedTurnBasedTileToolkit/Maps/Experimental/Hybrid/BP_ThirdPersonCharacter.BP_ThirdPersonCharacter_C|GetFollowCamera _asbp_third_person_character_2)))
  (bind _gridmanager_2 (Utilities|GetGridManager))
  (bind _outactors_2 (Actor|GetAllActorsOfClass "/Game/AdvancedTurnBasedTileToolkit/Maps/Experimental/Hybrid/BP_ThirdPersonCharacter.BP_ThirdPersonCharacter_C"))
  (for _array_element_2 _outactors_2
    (bind _asbp_unit (Utilities|Casting|CastToBP_Unit (Actor|GetParentActor _array_element_2)))
    (Utilities|QueueActionSingles _array_element_2 "Center" "NewEnumerator0" false -1 false 0.0 false 0 0.0 "" (+ (.Value (Utilities|Map|Find (Variables|/Game/AdvancedTurnBasedTileToolkit/Core/Grid/BP_GridManager.BP_GridManager_C|GetGridLocations _gridmanager_2) (Variables|/Game/AdvancedTurnBasedTileToolkit/Core/Grid/BP_GridActor.BP_GridActor_C|GetGridIndex _asbp_unit))) (Math|Vector|MakeVector 0.0 0.0 (Variables|/Script/Engine.CapsuleComponent|GetCapsuleHalfHeight (Variables|/Script/Engine.Character|GetCapsuleComponent _array_element_2))))))
  (CallFunction|BeginNewTurn))

(event Custom|EndTurnBasedMode
  (Default|CallOnTurnBasedEnd)
  (Class|BPIInitiative|DeselectActor(Message) (Variables|Default|GetActiveActor))
  (Utilities|SimpleQueue self "ShowSelection" "NewEnumerator0" true)
  (bind _actionmanager (Utilities|GetActionManager))
  (Default|InitializeQueuedActions _actionmanager)
  (Variables|Default|SetActivePlayer 0)
  (Utilities|FlowControl|Delay 1.0)
  (bind _returnvalue (Actor|GetActorOfClass "/Game/AdvancedTurnBasedTileToolkit/Maps/Experimental/Hybrid/BP_ThirdPersonCharacter.BP_ThirdPersonCharacter_C"))
  (Default|LerptoThirdPersonandPossess (Variables|Default|GetGridCameraRef) _returnvalue)
  (bind _asabp_hybrid (Utilities|Casting|CastToABP_Hybrid (Components|SkeletalMesh|GetAnimInstance (Variables|/Script/Engine.Character|GetMesh _returnvalue))))
  (Variables|/Game/AdvancedTurnBasedTileToolkit/Maps/Experimental/Hybrid/ABP_Hybrid.ABP_Hybrid_C|SetbThirdPerson _asabp_hybrid true))

(event EventStartMatch)

(event EventRunonActorDeselected
  (params (DeselectedActor :type Actor%20Object%20Reference))
  (Variables|Default|SetActiveActor 0)
  (bind _asbp_player_controller_atbtt (Utilities|Casting|CastToBP_PlayerController_ATBTT (Game|GetPlayerController 0)))
  (Default|Deactivate (Variables|/Game/AdvancedTurnBasedTileToolkit/Core/BP_PlayerController_ATBTT.BP_PlayerController_ATBTT_C|GetActiveAbility _asbp_player_controller_atbtt))
  (Variables|/Game/AdvancedTurnBasedTileToolkit/Core/BP_PlayerController_ATBTT.BP_PlayerController_ATBTT_C|SetActiveAbility _asbp_player_controller_atbtt 0))

(event EventNotifyPlayerReady
  (|CallParentFunction)
  (bind _asbp_grid_camera_hybrid (Utilities|Casting|CastToBP_GridCamera_Hybrid (Game|Player|GetPlayerPawn 0)))
  (Variables|Default|SetGridCameraRef _asbp_grid_camera_hybrid)
  (bind _returnvalue (Actor|GetActorOfClass "/Game/AdvancedTurnBasedTileToolkit/Maps/Experimental/Hybrid/BP_ThirdPersonCharacter.BP_ThirdPersonCharacter_C"))
  (Pawn|Possess (Game|GetPlayerController 0) _returnvalue))

(fn ConstructionScript
  (|CallParentFunction))

(fn EndGameifConditionMet
  (bind _bgameover (CallFunction|CheckifGameOver))
  (if _bgameover
    (bind _bgameover_2 (|CallParentFunction))
    (return _bgameover_2)
    (else
      (bind _actorsoffaction (CallFunction|FindInitiativeActorsOfFaction "NewEnumerator1"))
      (if (> (Utilities|Array|Length _actorsoffaction) 0)
        (return false)
        (else
          (CallFunction|EndTurnBasedMode)
          (return false))))))

(fn FindUnitsinSightOfActor
  (params (Actor :type Actor%20Object%20Reference))
  (bind _localunitactors (LocalVariables|GetLocalUnitActors))
  (bind _gridmanager (Utilities|GetGridManager))
  (bind _insightunits (Default|FindVisibleUnitsinRange _gridmanager (.Index (Default|ConvertLocationtoIndex3D _gridmanager (Transformation|GetActorLocation Actor))) 20 false 999999.0))
  (bind _result (Utilities|Set|ToArray _insightunits))
  (for _array_element _result
    (Utilities|Array|Add _localunitactors (.Value (Utilities|Map|Find (Variables|/Game/AdvancedTurnBasedTileToolkit/Core/Grid/BP_GridManager.BP_GridManager_C|GetGridUnits _gridmanager) _array_element))))
  (return _localunitactors))
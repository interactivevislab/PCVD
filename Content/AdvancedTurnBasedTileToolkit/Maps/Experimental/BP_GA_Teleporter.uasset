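; BP_GA_Teleporter is a grid actor for the turn-based tile toolkit that links its tile to a paired teleporter's tile.
; On BeginPlay it rebuilds CustomEdges as one edge of cost 1 to the partner, registers a special edge with the grid manager, then calls the parent.
; The link is one-way from this actor.
; The construction script calls the same helper without a partner, which only clears CustomEdges.
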(event EventBeginPlay
  (CallFunction|AddPairedTeleporterCustomEdge (Variables|Default|GetPairedTeleporter))
  (Default|AddSpecialEdge (Variables|Default|GetGridManagerRef) (Variables|Default|GetGridIndex) (Variables|/Game/AdvancedTurnBasedTileToolkit/Core/Grid/BP_GridActor.BP_GridActor_C|GetGridIndex (Variables|Default|GetPairedTeleporter)) "NewEnumerator4")
  (|CallParentFunction))

(fn ConstructionScript
  (CallFunction|AddPairedTeleporterCustomEdge)
  (|CallParentFunction))

(fn AddPairedTeleporterCustomEdge
  (params (InputPin :type BP%20GA%20Teleporter%20Object%20Reference))
  (Utilities|Array|Clear (Variables|Default|GetCustomEdges))
  (Utilities|IsValid InputPin
    (:Is%20Valid
      (Utilities|Array|Add (Variables|Default|GetCustomEdges) (Utilities|Struct|MakeFCustomEdge (Variables|Default|GetGridIndex) (Variables|/Game/AdvancedTurnBasedTileToolkit/Core/Grid/BP_GridActor.BP_GridActor_C|GetGridIndex InputPin) 1)))))
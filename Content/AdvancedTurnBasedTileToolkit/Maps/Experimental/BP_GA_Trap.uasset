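; Grid-placed trap for the turn-based tile toolkit that damages a unit interacting with it.
; It registers itself with the grid manager on BeginPlay, and Interact applies damage immediately with auto-animation off, storing the unit and path index.
; It binds to the grid manager's tile-enter animation event, so the "Hurt" action is queued only when that unit's animation reaches the stored path index, separating game logic from visual feedback.
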(event Custom|DisplayDamage
  (params (Unit :type BP%20Unit%20Object%20Reference) (PathIndex :type Integer))
  (if (and (== Unit (Variables|Default|GetTriggeringUnit)) (== PathIndex (Variables|Default|GetTriggeringPathIndex)))
    (Utilities|QueueActionSingles (Variables|Default|GetTriggeringUnit) "Hurt" "NewEnumerator2" false -1 false 0.0 false 0 (Variables|Default|GetDamage))))

(event EventInteract
  (params (TriggeringActor :type Actor%20Object%20Reference) (InteractionType :type EInteract%20Enum :default "NewEnumerator0") (CurrentPathIndex :type Integer))
  (bind _asbp_unit (Utilities|Casting|CastToBP_Unit TriggeringActor))
  (Variables|Default|SetTriggeringUnit _asbp_unit)
  (Variables|Default|SetTriggeringPathIndex CurrentPathIndex)
  (EventDispatchers|BindEventtoOnUnitEnterTileAnimate (Variables|Default|GetGridManagerRef) (delegate Custom|DisplayDamage))
  (Default|TakeDamage (Variables|Default|GetTriggeringUnit) (Variables|Default|GetDamage) false))

(event EventBeginPlay
  (Default|AddObjecttoGrid (Variables|Default|GetGridManagerRef) self (Variables|Default|GetGridIndex)))

(fn ConstructionScript)
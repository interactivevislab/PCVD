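; 2D Kraken unit for the turn-based tile toolkit that takes its tentacles with it when it dies.
; It overrides AnimateAction, deferring to the parent for every action and adding extra handling for Death.
; On Death, it queues every BP_GA_Tentacle actor in the level for destruction and swaps each tentacle's sprite to a random blood sprite.
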(event EventAnimateAction
  (params (Action :type F%20Action%20Structure))
  (bind _bloodsprites (Variables|Default|GetBloodSprites))
  (switch name (CallFunction|GetActionName Action)
    (:Default
      (|CallParentFunction Action :!label _label))
    (:Death
      (Utilities|FlowControl|Sequence
        (:then_0
          (goto _label))
        (:then_1
          (bind _outactors (Actor|GetAllActorsOfClass "/Game/AdvancedTurnBasedTileToolkit/Maps/2D/Units/BP_GA_Tentacle.BP_GA_Tentacle_C"))
          (Utilities|QueueDestroy _outactors)
          (for _array_element _outactors
            (Rendering|Components|Sprite|SetSprite (Variables|/Game/AdvancedTurnBasedTileToolkit/Maps/2D/Units/BP_GA_Tentacle.BP_GA_Tentacle_C|GetTentacleSprite _array_element) (Utilities|Array|Get(acopy) _bloodsprites (Math|Random|RandomIntegerinRange 0 (Utilities|Array|LastIndex _bloodsprites))))))))))

(fn ConstructionScript
  (|CallParentFunction))
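; Turn manager variant for the 2D Hydra map of the turn-based tile toolkit, customizing camera follow and the game-over message.
; AnimateAction replaces parent handling of Store Turn Info and Show Selection to make the player pawn follow the action's actor, with the former also caching turn and active actor.
; Other actions go to the parent.
; DisplayGameOver shows victory on the HUD if the remaining unit is exactly BP_Unit_2D_Hydra, otherwise game over.
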(event EventDisplayGameOver
  (params (RemainingUnit :type BP%20Unit%20Object%20Reference))
  (bind _asbp_hud_atbtt (Utilities|Casting|CastToBP_HUD_ATBTT (HUD|GetHUD (Game|GetPlayerController 0))))
  (if (== (Utilities|GetClass RemainingUnit) "/Game/AdvancedTurnBasedTileToolkit/Maps/2D/Units/BP_Unit_2D_Hydra.BP_Unit_2D_Hydra_C")
    (Default|DisplayCenterText (Variables|/Game/AdvancedTurnBasedTileToolkit/Core/UI/BP_HUD_ATBTT.BP_HUD_ATBTT_C|GetWbpAtbttRef _asbp_hud_atbtt) "VICTORY!" false 0.0)
    (else
      (Default|DisplayCenterText (Variables|/Game/AdvancedTurnBasedTileToolkit/Core/UI/BP_HUD_ATBTT.BP_HUD_ATBTT_C|GetWbpAtbttRef _asbp_hud_atbtt) "GAME OVER" false 0.0))))

(event EventAnimateAction
  (params (Action :type F%20Action%20Structure))
  (bind _actor (CallFunction|GetActor Action))
  (switch name (CallFunction|GetActionName Action)
    (:Default
      (|CallParentFunction Action))
    (:StoreTurnInfo
      (Variables|Default|SetCurrentTurnAnimate (CallFunction|GetInteger Action))
      (Variables|Default|SetActiveActorAnimate _actor)
      (Class|BPICameraControls|FollowActor(Message) (Game|Player|GetPlayerPawn 0) _actor :!label _label))
    (:ShowSelection
      (goto _label))))

(fn ConstructionScript
  (|CallParentFunction))
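; Interactable paired-torch item for the 2D turn-based tile toolkit that lights up and prompts bridges to raise.
; The first interaction calls AttemptRaise on every BP_GA_Bridge in the level and queues a "Light" action, guarded by DoOnce.
; AnimateAction toggles the lit and unlit visuals and plays the torch sound.
; The construction script positions the second torch's anchor from a configurable XY offset at a fixed height.
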(event EventInteract
  (params (TriggeringActor :type Actor%20Object%20Reference) (InteractionType :type EInteract%20Enum :default "NewEnumerator0") (CurrentPathIndex :type Integer))
  (Utilities|FlowControl|DoOnce false
    (:Completed
      (bind _outactors (Actor|GetAllActorsOfClass "/Game/AdvancedTurnBasedTileToolkit/Maps/2D/Tiles/BP_GA_Bridge.BP_GA_Bridge_C"))
      (for _array_element _outactors
        (Default|AttemptRaise _array_element))
      (Utilities|SimpleQueue self "Light" "NewEnumerator0" true))))

(event EventAnimateAction
  (params (Action :type F%20Action%20Structure))
  (Rendering|ToggleVisibility (Variables|Default|GetTorchUnlit) false)
  (Audio|PlaySound2D "/Game/AdvancedTurnBasedTileToolkit/Maps/2D/Items/A_Torch.A_Torch" 1.0 1.0 0.0 0 0))

(fn ConstructionScript
  (bind _pairedtorchoffset (Variables|Default|GetPairedTorchOffset))
  (|CallParentFunction)
  (Transformation|SetRelativeLocation (Variables|Default|GetPairedAnchor) (Math|Vector|MakeVector (.x _pairedtorchoffset) (.y _pairedtorchoffset) 5e+01) false false))
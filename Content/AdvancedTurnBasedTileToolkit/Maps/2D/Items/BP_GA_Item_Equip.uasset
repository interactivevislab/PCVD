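; Equippable item pickup for the 2D turn-based map that gives a hero unit new gear when interacted with.
; Interact accepts only 2D heroes and, once, passes the item's stats, sprite, type, sounds and projectile to Equip.
; It then queues its own Destroy action and a DestroyActors action on the action manager.
; AnimateAction handles the queued visuals, hiding the item and playing a potion sound.
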(event EventAnimateAction
  (params (Action :type F%20Action%20Structure))
  (switch name (CallFunction|GetActionName Action)
    (:Destroy
      (Rendering|SetActorHiddenInGame true)
      (Audio|PlaySound2D "/Game/AdvancedTurnBasedTileToolkit/Maps/2D/Items/A_Potion.A_Potion" 1.0 1.0 0.0 0 0))))

(event EventInteract
  (params (TriggeringActor :type Actor%20Object%20Reference) (InteractionType :type EInteract%20Enum :default "NewEnumerator0") (CurrentPathIndex :type Integer))
  (bind _asbp_unit_2d_hero (Utilities|Casting|CastToBP_Unit_2D_Hero TriggeringActor))
  (Utilities|FlowControl|DoOnce false
    (:Completed
      (Default|Equip _asbp_unit_2d_hero (Variables|Default|GetDamage) (Variables|Default|GetArmor) (Variables|Default|GetEquipSprite) (Variables|Default|GetEquipType) (Variables|Default|GetRange) (Variables|Default|GetAttackSound) (Variables|Default|GetHitSound) (Variables|Default|GetProjectile))
      (Utilities|SimpleQueue self "Destroy" "NewEnumerator0" true)
      (bind _actionmanager (Utilities|GetActionManager))
      (Utilities|QueueActionSingles :Executing%20Object _actionmanager :Action%20Name "DestroyActors" :Instant%20Deactivate true :Actor self))))

(fn ConstructionScript
  (|CallParentFunction))